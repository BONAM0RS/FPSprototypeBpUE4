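; Loot component that drops a BP_LootActor from its owner, optionally when the owner is destroyed.
; When HaveLootOnDestroy is set, BeginPlay binds the owner's destroyed event to SpawnRandomLoot.
; That event picks a random LootDataTable entry, recursively rerolling Ammo_Pistol, and spawns it at the owner's bounds origin with random yaw.
; SpawnLootDataTable spawns every entry instead, but its only call here is disconnected.
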(event Custom|SpawnLootDataTable
  (for _array_element (Variables|Default|GetLootDataTable)
    (Game|SpawnActorfromClass "/Game/-RLS_Project/Environment/Loot/BP_LootActor.BP_LootActor_C" (Math|Transform|MakeTransform (.Origin (Collision|GetActorBounds (Components|GetOwner) true false)) (Math|Rotator|MakeRotator 0.0 0.0 (Math|Random|RandomFloatinRange -1.8e+02 1.8e+02))) "Undefined" 0 _array_element 0)))

(event Custom|On%20Actor%20Destroyed
  (params (DestroyedActor :type Actor%20Object%20Reference))
  (CallFunction|SpawnRandomLoot))

(event Custom|SpawnRandomLoot
  (bind _lootdatatable (Variables|Default|GetLootDataTable))
  (Utilities|Array|Shuffle _lootdatatable)
  (bind _output_get (Variables|Default|SetLoot (.OutItem (Utilities|Array|Random _lootdatatable))))
  (if (Utilities|Name|NotEqual(Name) (.RowName (Utilities|Struct|BreakDataTableRowHandle _output_get)) "Ammo_Pistol")
    (Game|SpawnActorfromClass "/Game/-RLS_Project/Environment/Loot/BP_LootActor.BP_LootActor_C" (Math|Transform|MakeTransform (.Origin (Collision|GetActorBounds (Components|GetOwner) true false)) (Math|Rotator|MakeRotator 0.0 0.0 (Math|Random|RandomFloatinRange -1.8e+02 1.8e+02))) "Undefined" 0 (Variables|Default|GetLoot) 0)
    (else
      (CallFunction|SpawnRandomLoot))))

(event EventBeginPlay
  (if (Variables|Default|GetHaveLootOnDestroy)
    (Game|BindEventtoOnDestroyed (Components|GetOwner) (delegate Custom|On%20Actor%20Destroyed))))