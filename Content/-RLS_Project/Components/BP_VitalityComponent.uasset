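; Actor component that manages its owner's health, damage intake, regeneration and death.
; It binds to the owner's point and radial damage events, ignores hits on excluded components and scales damage by per-type multipliers from BP_DamageType_Base.
; Successful non-lethal hits restart a delayed looping timer that heals a percentage of total HP until full, if regen is enabled.
; HP changes and death are broadcast through OnChangedHP and OnDied dispatchers.
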(event Custom|PointDamage
  (params (DamagedActor :type Actor%20Object%20Reference) (Damage :type Float%20%28single-precision%29) (InstigatedBy :type Controller%20Object%20Reference) (HitLocation :type Vector) (FHitComponent :type Primitive%20Component%20Object%20Reference) (BoneName :type Name) (ShotFromDirection :type Vector) (DamageType :type Damage%20Type%20Object%20Reference) (DamageCauser :type Actor%20Object%20Reference))
  (if (not (Utilities|Array|ContainsItem (Variables|Default|GetNoDamageComponents) FHitComponent))
    (bind _isdamaged (CallFunction|ApplyDamage Damage DamageType))
    (if _isdamaged
      (CallFunction|CheckRegen))))

(event Custom|RadialDamage
  (params (DamagedActor :type Actor%20Object%20Reference) (Damage :type Float%20%28single-precision%29) (DamageType :type Damage%20Type%20Object%20Reference) (Origin :type Vector) (HitInfo :type Hit%20Result%20Structure) (InstigatedBy :type Controller%20Object%20Reference) (DamageCauser :type Actor%20Object%20Reference))
  (if (not (Utilities|Array|ContainsItem (Variables|Default|GetNoDamageComponents) (.HitComponent (Collision|BreakHitResult HitInfo))))
    (bind _isdamaged (CallFunction|ApplyDamage Damage DamageType))
    (if _isdamaged
      (CallFunction|CheckRegen))))

(event Custom|Apply%20Regen
  (CallFunction|ApplyHeal (* (* (/ (Variables|-HP|GetRegenPercentPerSec) 1e+02) (Variables|-HP|GetTotalHP)) (Variables|-HP|GetRegenTickDelay)))
  (if (>= (Variables|-HP|GetCurrentHP) (Variables|-HP|GetTotalHP))
    (Utilities|Time|ClearandInvalidateTimerbyHandle (Variables|Default|GetRegenTimerHandle))))

(event Custom|Check%20Regen
  (if (Variables|-Params|GetHaveRegen)
    (Utilities|Time|ClearandInvalidateTimerbyHandle (Variables|Default|GetRegenTimerHandle))
    (if (not (Variables|Default|GetIsDead))
      (bind _returnvalue (Utilities|Time|SetTimerbyEvent (delegate Custom|Apply%20Regen) (Variables|-HP|GetRegenTickDelay) true (- (Variables|-HP|GetRegenStartDelay) (Variables|-HP|GetRegenTickDelay))))
      (Variables|Default|SetRegenTimerHandle _returnvalue))))

(event EventBeginPlay
  (bind _returnvalue (Components|GetOwner))
  (EventDispatchers|BindEventtoOnTakePointDamage _returnvalue (delegate Custom|PointDamage))
  (EventDispatchers|BindEventtoOnTakeRadialDamage _returnvalue (EventDispatchers|CreateEvent :!event Custom|RadialDamage))
  (Variables|-HP|SetCurrentHP (Variables|-HP|GetTotalHP)))

(fn ApplyDamage
  (params (Damage :type Float%20%28single-precision%29) (DamageType :type Damage%20Type%20Object%20Reference))
  (LocalVariables|SetLocal_ActualDamage Damage)
  (Utilities|FlowControl|Sequence
    (:then_0
      ;[1 1 1] Apply Damage Multiplier
      (bind _asbp_damage_type_base (Utilities|Casting|CastToBP_DamageType_Base DamageType))
      (if (.ReturnValue (Utilities|Map|Find (Variables|Default|GetDamageTypeMulti) (Variables|/Game/-RLS_Project/Weapons/DamageTypes/BP_DamageType_Base.BP_DamageType_Base_C|GetDamageType _asbp_damage_type_base)))
        (LocalVariables|SetLocal_ActualDamage (* (.Value (Utilities|Map|Find (Variables|Default|GetDamageTypeMulti) (Variables|/Game/-RLS_Project/Weapons/DamageTypes/BP_DamageType_Base.BP_DamageType_Base_C|GetDamageType _asbp_damage_type_base))) (LocalVariables|GetLocal_ActualDamage)))))
    (:then_1
      ;[1 1 1] Apply Actual Damage
      (if (> (LocalVariables|GetLocal_ActualDamage) 0.0)
        (bind _output_get (Variables|-HP|SetCurrentHP (Math|Float|Clamp(Float) (- (Variables|-HP|GetCurrentHP) (LocalVariables|GetLocal_ActualDamage)) 0.0 (Variables|-HP|GetTotalHP))))
        (Default|CallOnChangedHP _output_get (Variables|-HP|GetTotalHP))
        (LocalVariables|SetIsDamage true)
        (else
          (LocalVariables|SetIsDamage false))))
    (:then_2
      ;[1 1 1] Apply Death
      (if (< (Variables|-HP|GetCurrentHP) 1.0)
        (if (Variables|-Params|GetCanDie)
          (if (not (Variables|Default|GetIsDead))
            (Variables|Default|SetIsDead true)
            (Default|CallOnDied)))
        (else
          (return (LocalVariables|GetIsDamage)))))))

(fn ApplyHeal
  (params (RegenHP :type Float%20%28single-precision%29))
  (if (< (Variables|-HP|GetCurrentHP) (Variables|-HP|GetTotalHP))
    (bind _output_get (Variables|-HP|SetCurrentHP (Math|Float|Clamp(Float) (+ (Variables|-HP|GetCurrentHP) RegenHP) 0.0 (Variables|-HP|GetTotalHP))))
    (Default|CallOnChangedHP _output_get (Variables|-HP|GetTotalHP))))