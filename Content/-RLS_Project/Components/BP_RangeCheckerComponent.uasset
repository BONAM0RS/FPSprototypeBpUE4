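; Range checker component that fires catch and release events as the player camera moves near or away from its owning actor.
; Each Tick measures camera-to-owner distance, calling OnCatch inside CatchRadius and OnRelease beyond ReleaseRadius.
; The IsCatch flag alternates the two checks, so each event fires once per crossing, with separate radii allowing hysteresis.
; DeactivateTick sets IsDead, which permanently skips the check without disabling Tick itself.
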(event Custom|DeactivateTick
  (Variables|Default|SetIsDead true))

(event EventBeginPlay)

(event EventTick
  (params (DeltaSeconds :type Float%20%28single-precision%29))
  (if (not (Variables|Default|GetIsDead))
    (Variables|Default|SetDistance (Math|Vector|VectorLength (- (Camera|GetCameraLocation (Game|GetPlayerCameraManager 0)) (Transformation|GetActorLocation (Components|GetOwner)))))
    (if (Variables|Default|GetIsCatch)
      (if (< (Variables|Default|GetDistance) (Variables|Default|GetCatchRadius))
        (Variables|Default|SetIsCatch false)
        (Default|CallOnCatch))
      (elif (> (Variables|Default|GetDistance) (Variables|Default|GetReleaseRadius))
        (Variables|Default|SetIsCatch true)
        (Default|CallOnRelease)))))