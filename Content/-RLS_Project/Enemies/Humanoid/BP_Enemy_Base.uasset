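; Base humanoid enemy character that patrols, attacks, shows health in a widget and scales HP with game difficulty.
; It spawns a socketed weapon and loops AI moves between spawn and patrol points while its logic flag is off.
; Attacks either fire ranged shots and close on the player or play random montages, then signal completion.
; Death triggers ragdoll, weapon physics and optional random loot, then delayed destruction.
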(event OnChangedHP(BP_VitalityComponent)
  (params (CurrentHP :type Float%20%28single-precision%29) (TotalHP :type Float%20%28single-precision%29))
  ;[1 1 1] Widget HP
  (bind _aswbp_enemy_hp (Utilities|Casting|CastToWBP_EnemyHP (UserInterface|GetUserWidgetObject (Variables|Default|GetWidget_HP))))
  (Default|SetHP _aswbp_enemy_hp CurrentHP TotalHP))

(event OnDied(BP_VitalityComponent)
  (bind _currentweapon (Variables|Default|GetCurrentWeapon))
  (bind _currentweapon_2 (Variables|Default|GetCurrentWeapon))
  ;[1 1 1] Death Process
  (Utilities|FlowControl|Sequence
    (:then_0
      (Collision|SetCollisionProfileName (Variables|Character|GetMesh) "Ragdoll" true :!class /Script/Engine.PrimitiveComponent)
      (Physics|SetSimulatePhysics (Variables|Character|GetMesh) true))
    (:then_1
      (Collision|SetCollisionEnabled (Variables|Collision|GetCapsuleComponent) "NoCollision"))
    (:then_2
      (Utilities|IsValid _currentweapon_2
        (:Is%20Valid
          (Default|ApplyWeaponPhysicsonDeath _currentweapon_2))))
    (:then_3
      (if (Variables|Default|GetHaveLootOnDeath)
        (Default|SpawnRandomLoot (Variables|Default|GetBP_LootComponent))))
    (:then_4
      (Utilities|FlowControl|Delay 1e+01)
      (Utilities|FlowControl|Sequence
        (:then_0
          (Actor|DestroyActor))
        (:then_1
          (Utilities|FlowControl|Delay 3e+01)
          (Utilities|IsValid _currentweapon
            (:Is%20Valid
              (Actor|DestroyActor _currentweapon))))))))

(event Custom|StartAttack
  ;[1 1 1] AI Controller
  (if (Variables|Default|GetIsRange)
    (bind _result (Default|TryMakeShot (Variables|Default|GetCurrentWeapon)))
    (if _result
      (AI|AIMoveTo (Class|PawnMovementComponent|GetPawnOwner (Variables|Character|GetCharacterMovement)) "0, 0, 0" (Game|GetPlayerCharacter 0) 1e+02 false
        (:then
          (Utilities|FlowControl|Delay 1.0)
          (CallFunction|StartAttack)))
      (else
        (Animation|Montage|PlayMontage (Variables|Character|GetMesh) (.OutItem (Utilities|Array|Random (Variables|-AttackSettings|GetAttackMontages))) :!label _label
          (:OnBlendOut
            _)
          (:OnInterrupted
            _))
        (Default|CallOnAttackFinished)))
    (else
      (goto _label))))

(event Custom|SpawnWeapon
  (bind _returnvalue (Game|SpawnActorfromClass (Variables|Default|GetWeaponClass) (Math|Transform|MakeTransform "0, 0, 0" "0, 0, 0" "1,1,1") "Undefined" self 0))
  (bind _output_get (Variables|Default|SetCurrentWeapon _returnvalue))
  (Utilities|IsValid _output_get
    (:Is%20Valid
      (Transformation|AttachComponentToComponent _output_get (Variables|Character|GetMesh) (Utilities|Select :Index (Variables|Default|GetEnemyWeapon) :NewEnumerator0 "Hand_RSocket" :NewEnumerator3 "Hand_RSocket_Club" :NewEnumerator4 "Hand_RSocket_Axe" :NewEnumerator5 "Hand_RSocket_Crowbar" :NewEnumerator1 "Hand_RSocket" :NewEnumerator6 "Hand_RSocket" :NewEnumerator10 "Hand_RSocket" :NewEnumerator7 "Hand_RSocket" :NewEnumerator8 "Hand_RSocket" :NewEnumerator9 "Hand_RSocket") "SnapToTarget" "SnapToTarget" "SnapToTarget" true))))

(event Custom|MoveToPatrolLocation
  ;[1 1 1] AI Controller
  (if (not (Variables|Default|GetIsLogicActive))
    (AI|SetFocus (AI|GetAIController self))
    (AI|AIMoveTo (Class|PawnMovementComponent|GetPawnOwner (Variables|Character|GetCharacterMovement)) (Variables|-PatrolSettings|GetPatrolLocation) 0 1.5e+02 false
      (:OnSuccess
        (Utilities|FlowControl|Delay 2.0)
        (CallFunction|MovetoSpawnLocation))
      (:OnFail
        (Utilities|FlowControl|Delay 1.0)
        (CallFunction|MovetoPatrolLocation)))))

(event Custom|MoveToSpawnLocation
  ;[1 1 1] AI Controller
  (if (not (Variables|Default|GetIsLogicActive))
    (AI|SetFocus (AI|GetAIController self))
    (AI|AIMoveTo (Class|PawnMovementComponent|GetPawnOwner (Variables|Character|GetCharacterMovement)) (Variables|Default|GetSpawnLocation) 0 5e+01 false
      (:OnSuccess
        (Utilities|FlowControl|Delay 2.0)
        (CallFunction|MovetoPatrolLocation))
      (:OnFail
        (Utilities|FlowControl|Delay 1.0)
        (CallFunction|MovetoSpawnLocation)))))

(event Custom|CheckActivateLogic
  (params (IsLogicActive :type Boolean))
  ;[1 1 1] AI Controller
  (Variables|Default|SetIsLogicActive IsLogicActive))

(event EventBeginPlay
  (bind _bp_vitalitycomponent (Variables|Default|GetBP_VitalityComponent))
  (CallFunction|SpawnWeapon)
  (bind _output_get (Variables|Default|SetSpawnLocation (Transformation|GetWorldLocation (Variables|Collision|GetCapsuleComponent))))
  (Variables|-PatrolSettings|SetPatrolLocation (+ _output_get (Variables|-PatrolSettings|GetPatrolLocation)))
  (bind _output_get_2 (Variables|/Game/-RLS_Project/Components/BP_VitalityComponent.BP_VitalityComponent_C|SetTotalHP _bp_vitalitycomponent (+ (Math|Conversions|ToFloat(Integer) (Utilities|Select :Index (Variables|/Game/-RLS_Project/Core/BP_GameInstance.BP_GameInstance_C|GetGameDifficulty (.AsBP%20Game%20Instance (Utilities|Casting|CastToBP_GameInstance (Game|GetGameInstance)))) :Option%200 0 :Option%201 50 :Option%202 100)) (Variables|/Game/-RLS_Project/Components/BP_VitalityComponent.BP_VitalityComponent_C|GetTotalHP (Variables|Default|GetBP_VitalityComponent)))))
  (Variables|/Game/-RLS_Project/Components/BP_VitalityComponent.BP_VitalityComponent_C|SetCurrentHP _bp_vitalitycomponent _output_get_2))

(event EventTick
  (params (DeltaSeconds :type Float%20%28single-precision%29))
  (Transformation|SetWorldRotation (Variables|Default|GetArrow_AIController) (Pawn|GetControlRotation :!class /Script/Engine.Pawn) false false))

(fn ConstructionScript)