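; Enemy turret bullet projectile that deals point damage to what it hits and destroys itself after a two-second lifetime.
; A sphere collision hit destroys the bullet without damage on Enemy-tagged actors and routes other valid actors to HitTarget.
; HitTarget runs once, spawning an impact emitter and quiet sound, applying damage along the trace direction, then destroying the bullet.
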(event OnComponentHit(Sphere)
  (params (HitComponent :type Primitive%20Component%20Object%20Reference) (OtherActor :type Actor%20Object%20Reference) (OtherComp :type Primitive%20Component%20Object%20Reference) (NormalImpulse :type Vector :default "0, 0, 0") (Hit :type Hit%20Result%20Structure%20%28by%20ref%29))
  (Utilities|IsValid OtherActor
    (:Is%20Valid
      (if (not (Actor|ActorHasTag OtherActor "Enemy"))
        (CallFunction|HitTarget OtherActor Hit)
        (else
          (Actor|DestroyActor))))))

(event Custom|HitTarget
  (params (HitActor :type Actor%20Object%20Reference) (HitResult :type Hit%20Result%20Structure))
  (bind _returnvalue (Transformation|GetActorLocation))
  (bind (_bblockinghit _binitialoverlap _time _distance _location _impactpoint _normal _impactnormal _physmat _hitactor _hitcomponent _hitbonename _hititem _elementindex _faceindex _tracestart _traceend) (Collision|BreakHitResult HitResult))
  (Utilities|FlowControl|DoOnce false
    (:Completed
      (Utilities|FlowControl|Sequence
        (:then_0
          (Effects|SpawnEmitteratLocation 0 _returnvalue)
          (Audio|SpawnSoundatLocation 0 _returnvalue "0, 0, 0" 0.1 1.0 0.0 0 0))
        (:then_1
          (Game|Damage|ApplyPointDamage HitActor (Variables|Default|GetDamage) (Math|Vector|Normalize (- _traceend _tracestart)) HitResult))
        (:then_2
          (Actor|DestroyActor))))))

(event EventBeginPlay
  (|CallParentFunction)
  (Utilities|FlowControl|Delay 2.0)
  (Actor|DestroyActor))

(fn ConstructionScript
  (|CallParentFunction))