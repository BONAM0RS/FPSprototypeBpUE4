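; Base weapon for humanoid enemies, handling melee, hitscan and projectile attacks, with a damage bonus from game difficulty.
; Animation-driven melee toggles a collision box that damages each overlapped non-enemy actor once per activation.
; Ranged attacks sphere-trace from the muzzle arrow toward the player camera, then apply point damage or spawn an aimed bullet or grenade.
; TryMakeShot reports whether that line is blocked, and death turns the mesh into a physics object.
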(event OnComponentBeginOverlap(DamageCollision)
  (params (OverlappedComponent :type Primitive%20Component%20Object%20Reference) (OtherActor :type Actor%20Object%20Reference) (OtherComp :type Primitive%20Component%20Object%20Reference) (OtherBodyIndex :type Integer) (bFromSweep :type Boolean) (SweepResult :type Hit%20Result%20Structure%20%28by%20ref%29))
  (bind _returnvalue (Components|GetOwner))
  (if (and (not (Actor|ActorHasTag OtherActor "Enemy")) (!= OtherActor _returnvalue))
    (bind _newparam (CallFunction|CheckCollisionHit OtherActor))
    (if _newparam
      (Game|Damage|ApplyPointDamage OtherActor (Variables|Default|GetDamage) (Math|Vector|Normalize (- (Transformation|GetActorLocation OtherActor) (Transformation|GetActorLocation _returnvalue))) SweepResult 0 self))))

(event Custom|ApplyWeaponPhysicsOnDeath
  (bind _weaponmesh (Variables|Default|GetWeaponMesh))
  (Collision|SetCollisionEnabled (Variables|Default|GetDamageCollision) "NoCollision")
  (Collision|SetCollisionProfileName _weaponmesh "PhysicsActor" true :!class /Script/Engine.PrimitiveComponent)
  (Physics|SetSimulatePhysics _weaponmesh true))

(event Custom|ActivateDamageCollision
  (params (On%20Off :type Boolean))
  (Collision|SetCollisionEnabled (Variables|Default|GetDamageCollision) (select On%20Off "QueryOnly" "NoCollision"))
  (Utilities|Array|Clear (Variables|Default|GetDamagedActors)))

(event Custom|FireHitScan
  (bind _returnvalue (Game|GetPlayerCameraManager 0))
  (bind _arrow (Variables|Default|GetArrow))
  (bind _returnvalue_2 (Transformation|GetWorldLocation _arrow))
  (bind _returnvalue_3 (Camera|GetCameraLocation _returnvalue))
  (bind _returnvalue_4 (- _returnvalue_3 "0, 0,10.000000"))
  (bind _outhit (Collision|SphereTraceByChannel _returnvalue_2 _returnvalue_4 5.0 "TraceTypeQuery1" false 0 "None" true "(R=1.000000,G=0.000000,B=0.000000,A=1.000000)" "(R=0.000000,G=1.000000,B=0.000000,A=1.000000)" 0.0))
  (Rendering|Debug|DrawDebugLine _returnvalue_2 _returnvalue_4 "(R=0.458333,G=0.458333,B=0.458333,A=1.000000)" 0.02 1.0)
  (Game|SpawnActorfromClass "/Game/-RLS_Project/Environment/ImpactEffect/BP_ImpactEffect.BP_ImpactEffect_C" (Math|Transform|MakeTransform _returnvalue_4 "0, 0, 0" "1,1,1") "Undefined" 0 _outhit 0)
  (Game|Damage|ApplyPointDamage (.HitActor (Collision|BreakHitResult _outhit)) (Variables|Default|GetDamage) (Math|Vector|Normalize (- (.TraceEnd (Collision|BreakHitResult _outhit)) (.TraceStart (Collision|BreakHitResult _outhit)))) _outhit (AI|GetAIController self) (Game|GetPlayerController 0) (Variables|Default|GetDamageType))
  (Components|Activation|Activate (Variables|Default|GetSound) true))

(event Custom|FireProjectile
  (bind _returnvalue (Game|GetPlayerCameraManager 0))
  (bind _returnvalue_2 (Components|GetOwner))
  (bind _returnvalue_3 (Components|GetOwner))
  (bind _arrow (Variables|Default|GetArrow))
  (bind _arrow_2 (Variables|Default|GetArrow))
  (bind _returnvalue_4 (Transformation|GetWorldTransform _arrow))
  (bind _returnvalue_5 (Transformation|GetWorldLocation _arrow_2))
  (bind _returnvalue_6 (Camera|GetCameraLocation _returnvalue))
  (bind _asbp_enemy_base (Utilities|Casting|CastToBP_Enemy_Base _returnvalue_3))
  (bind _asbp_enemy_base_2 (Utilities|Casting|CastToBP_Enemy_Base _returnvalue_2))
  (bind _returnvalue_7 (- _returnvalue_6 "0, 0,5.000000"))
  (bind _currentweapon (Variables|/Game/-RLS_Project/Enemies/Humanoid/BP_Enemy_Base.BP_Enemy_Base_C|GetCurrentWeapon _asbp_enemy_base))
  (bind _currentweapon_2 (Variables|/Game/-RLS_Project/Enemies/Humanoid/BP_Enemy_Base.BP_Enemy_Base_C|GetCurrentWeapon _asbp_enemy_base_2))
  (bind _outhit (Collision|SphereTraceByChannel _returnvalue_5 _returnvalue_7 5.0 "TraceTypeQuery1" false 0 "None" true "(R=1.000000,G=0.000000,B=0.000000,A=1.000000)" "(R=0.000000,G=1.000000,B=0.000000,A=1.000000)" 1.0))
  (Rendering|Debug|DrawDebugLine _returnvalue_5 _returnvalue_7 "(R=0.458333,G=0.458333,B=0.458333,A=1.000000)" 0.02 0.5)
  (if (Variables|Default|GetIsBullet)
    (bind _returnvalue_8 (Game|SpawnActorfromClass "/Game/-RLS_Project/Enemies/Humanoid/Weapons/Projectiles/BP_Projectile_EnemyBullet.BP_Projectile_EnemyBullet_C" (Math|Transform|MakeTransform (.location _returnvalue_4) (Math|Rotator|FindLookatRotation (.location _returnvalue_4) (select (.bBlockingHit (Collision|BreakHitResult _outhit)) (.ImpactPoint (Collision|BreakHitResult _outhit)) (.TraceEnd (Collision|BreakHitResult _outhit)))) "1,1,1") "Undefined" 0 0))
    (Variables|/Game/-RLS_Project/Weapons/Projectiles/BP_Projectile_Base.BP_Projectile_Base_C|SetDamage _returnvalue_8 (Variables|BP_PawnWeapon_Base_C|GetDamage _currentweapon_2))
    (Variables|/Game/-RLS_Project/Weapons/Projectiles/BP_Projectile_Base.BP_Projectile_Base_C|SetDamageType _returnvalue_8 (Variables|BP_PawnWeapon_Base_C|GetDamageType _currentweapon_2))
    (Components|Activation|Activate (Variables|Default|GetSound) true)
    (else
      (bind _returnvalue_9 (Game|SpawnActorfromClass "/Game/-RLS_Project/Enemies/Humanoid/Weapons/Projectiles/BP_Projectile_EnemyGrenade.BP_Projectile_EnemyGrenade_C" (Math|Transform|MakeTransform (.location _returnvalue_4) (Math|Rotator|FindLookatRotation (.location _returnvalue_4) (select (.bBlockingHit (Collision|BreakHitResult _outhit)) (.ImpactPoint (Collision|BreakHitResult _outhit)) (.TraceEnd (Collision|BreakHitResult _outhit)))) "1,1,1") "Undefined" 0 0))
      (Variables|/Game/-RLS_Project/Weapons/Projectiles/BP_Projectile_Base.BP_Projectile_Base_C|SetDamage _returnvalue_9 (Variables|BP_PawnWeapon_Base_C|GetDamage _currentweapon))
      (Variables|/Game/-RLS_Project/Weapons/Projectiles/BP_Projectile_Base.BP_Projectile_Base_C|SetDamageType _returnvalue_9 (Variables|BP_PawnWeapon_Base_C|GetDamageType _currentweapon))
      (Components|Activation|Activate (Variables|Default|GetSound) true))))

(event EventBeginPlay
  (Variables|Default|SetDamage (+ (Variables|Default|GetDamage) (Math|Conversions|ToFloat(Integer) (Utilities|Select :Index (Variables|/Game/-RLS_Project/Core/BP_GameInstance.BP_GameInstance_C|GetGameDifficulty (.AsBP%20Game%20Instance (Utilities|Casting|CastToBP_GameInstance (Game|GetGameInstance)))) :Option%200 0 :Option%201 5 :Option%202 10)))))

(event Collision|EventActorBeginOverlap
  (params (OtherActor :type Actor%20Object%20Reference)))

(event EventTick
  (params (DeltaSeconds :type Float%20%28single-precision%29)))

(fn ConstructionScript)

(fn CheckCollisionHit
  (params (Actor :type Actor%20Object%20Reference))
  (if (Utilities|Array|ContainsItem (Variables|Default|GetDamagedActors) 0)
    (return false)
    (else
      (Utilities|Array|Add (Variables|Default|GetDamagedActors) Actor)
      (return true))))

(fn TryMakeShot
  (bind _outhit (Collision|SphereTraceByChannel (Transformation|GetWorldLocation (Variables|Default|GetArrow)) (- (Camera|GetCameraLocation (Game|GetPlayerCameraManager 0)) "0, 0,20.000000") 5.0 "TraceTypeQuery1" false 0 "None" true "(R=1.000000,G=0.000000,B=0.000000,A=1.000000)" "(R=0.000000,G=1.000000,B=0.000000,A=1.000000)" 0.0))
  (return (.bBlockingHit (Collision|BreakHitResult _outhit))))