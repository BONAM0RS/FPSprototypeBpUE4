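; Rocket projectile, judging by its name fired by the turret enemy, that explodes on impact or two seconds after spawning.
; Both triggers call a DoOnce-guarded Explode event that spawns particles, sound and a camera shake at its location.
; It then applies radial damage with falloff, scaled by the Damage and Radius values and filtered by a prevention trace channel, before destroying itself.
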(event OnComponentHit(Sphere)
  (params (HitComponent :type Primitive%20Component%20Object%20Reference) (OtherActor :type Actor%20Object%20Reference) (OtherComp :type Primitive%20Component%20Object%20Reference) (NormalImpulse :type Vector :default "0, 0, 0") (Hit :type Hit%20Result%20Structure%20%28by%20ref%29))
  (CallFunction|Explode))

(event Custom|Explode
  (bind _returnvalue (Transformation|GetActorLocation))
  (bind _radius (Variables|Default|GetRadius))
  (bind _radius_2 (Variables|Default|GetRadius))
  (bind _damage (Variables|Default|GetDamage))
  (Utilities|FlowControl|DoOnce false
    (:Completed
      (Utilities|FlowControl|Sequence
        (:then_0
          (Effects|SpawnEmitteratLocation "/Game/MilitaryWeapDark/FX/P_Grenade_Explosion_01.P_Grenade_Explosion_01" _returnvalue)
          (Audio|SpawnSoundatLocation "/Game/MilitaryWeapDark/Sound/GrenadeLauncher/GrenadeLauncher_Explosion_Cue.GrenadeLauncher_Explosion_Cue" _returnvalue "0, 0, 0" 0.1 1.0 0.0 0 0)
          (Camera|PlayWorldCameraShake "/Game/-RLS_Project/Weapons/Projectiles/BP_Explosion_CamShake_Matinee.BP_Explosion_CamShake_Matinee_C" _returnvalue (/ _radius 3.0) _radius 1.0 true))
        (:then_1
          (Class|GameplayStatics|ApplyRadialDamagewithFalloff _damage (/ _damage 5.0) (Transformation|GetActorLocation) (/ _radius_2 3.0) _radius_2 1.0 (Variables|Default|GetDamageType) 0 0 0 "ECC_GameTraceChannel3"))
        (:then_2
          (Actor|DestroyActor))))))

(event EventBeginPlay
  (|CallParentFunction)
  (Utilities|FlowControl|Delay 2.0)
  (CallFunction|Explode))

(fn ConstructionScript
  (|CallParentFunction))