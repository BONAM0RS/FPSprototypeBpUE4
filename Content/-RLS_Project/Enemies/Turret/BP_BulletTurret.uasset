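; Enemy twin-barrel bullet turret that spins idly until its range checker catches a target, then tracks the player camera with split base yaw and barrel pitch.
; A delayed TryFire loop shoots projectiles from both muzzles when sphere traces are clear, though only the second trace's result counts.
; Game difficulty adds damage and HP at BeginPlay.
; The vitality component updates the HP widget and triggers death: explosion, physics collapse, optional loot, delayed destroy.
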(event OnCatch(BP_RangeChecker)
  ;[1 1 1] RANGE CHECK & FIRE
  (Variables|Default|SetIsCatched true)
  (Utilities|FlowControl|Delay 1.0)
  (CallFunction|TryFire))

(event OnRelease(BP_RangeChecker)
  ;[1 1 1] RANGE CHECK & FIRE
  (Variables|Default|SetIsCatched false))

(event OnChangedHP(BP_VitalityComponent)
  (params (CurrentHP :type Float%20%28single-precision%29) (TotalHP :type Float%20%28single-precision%29))
  ;[1 1 1] Widget HP
  (bind _aswbp_enemy_hp (Utilities|Casting|CastToWBP_EnemyHP (UserInterface|GetUserWidgetObject (Variables|Default|GetWidget_HP))))
  (Default|SetHP _aswbp_enemy_hp CurrentHP TotalHP))

(event OnDied(BP_VitalityComponent)
  ;[1 1 1] Vitality Component
  (Utilities|FlowControl|Sequence
    (:then_0
      (Variables|Default|SetIsDead true)
      (Default|DeactivateTick (Variables|Default|GetBP_RangeChecker))
      (Components|Activation|Activate (Variables|Default|GetExplosionVFX) true))
    (:then_1
      (Collision|SetCollisionProfileName (Variables|Default|GetBurrel) "PhysicsActor" true :!class /Script/Engine.PrimitiveComponent)
      (Physics|SetSimulatePhysics (Variables|Default|GetSphere) true))
    (:then_2
      (if (Variables|Default|GetHaveLootOnDeath)
        (Default|SpawnRandomLoot (Variables|Default|GetBP_LootComponent))))
    (:then_3
      (Utilities|FlowControl|Delay 1e+01)
      (Actor|DestroyActor))))

(event Custom|TryFire
  ;[1 1 1] RANGE CHECK & FIRE
  (if (not (Variables|Default|GetIsDead))
    (if (Variables|Default|GetIsCatched)
      (Utilities|IsValid (Game|GetPlayerCharacter 0)
        (:Is%20Valid
          (bind _israycasted (CallFunction|Raycast))
          (if _israycasted
            (Utilities|FlowControl|Delay (Variables|Default|GetAttackReload))
            (CallFunction|TryFire)
            (elif (not (Variables|Default|GetIsDead))
              (CallFunction|Fire)
              (Utilities|FlowControl|Delay (Variables|Default|GetAttackReload))
              (CallFunction|TryFire))))))))

(event EventBeginPlay
  (bind _returnvalue (Game|GetGameInstance))
  (bind _bp_vitalitycomponent (Variables|Default|GetBP_VitalityComponent))
  (bind _asbp_game_instance (Utilities|Casting|CastToBP_GameInstance _returnvalue))
  (bind _gamedifficulty (Variables|/Game/-RLS_Project/Core/BP_GameInstance.BP_GameInstance_C|GetGameDifficulty _asbp_game_instance))
  (Variables|Default|SetTurretDamage (+ (Variables|Default|GetTurretDamage) (Math|Conversions|ToFloat(Integer) (Utilities|Select :Index _gamedifficulty :Option%200 0 :Option%201 1 :Option%202 2))))
  (bind _output_get (Variables|/Game/-RLS_Project/Components/BP_VitalityComponent.BP_VitalityComponent_C|SetTotalHP _bp_vitalitycomponent (+ (Math|Conversions|ToFloat(Integer) (Utilities|Select :Index _gamedifficulty :Option%200 0 :Option%201 50 :Option%202 100)) (Variables|/Game/-RLS_Project/Components/BP_VitalityComponent.BP_VitalityComponent_C|GetTotalHP (Variables|Default|GetBP_VitalityComponent)))))
  (Variables|/Game/-RLS_Project/Components/BP_VitalityComponent.BP_VitalityComponent_C|SetCurrentHP _bp_vitalitycomponent _output_get))

(event EventTick
  (params (DeltaSeconds :type Float%20%28single-precision%29))
  (bind _returnvalue (Game|GetPlayerCameraManager 0))
  (bind _returnvalue_2 (Transformation|GetActorTransform))
  (bind _rootturret (Variables|Default|GetRootTurret))
  (bind _returnvalue_3 (Camera|GetCameraLocation _returnvalue))
  (bind _returnvalue_4 (- _returnvalue_3 "0, 0,20.000000"))
  ;[1 1 1] IDLE_STATE
  (if (Variables|Default|GetIsCatched)
    (if false
      ;[1 1 1] ATTACK_STATE (SIMPLE REALIZATION)
      (Transformation|SetWorldRotation _rootturret (Math|Rotator|FindLookatRotation (Transformation|GetWorldLocation _rootturret) (- (Camera|GetCameraLocation (Game|GetPlayerCameraManager 0)) "0, 0,20.000000")) false false)
      (else
        ;[1 1 1] ATTACK_STATE (HARD REALIZATION)
        (Transformation|SetRelativeRotation (Variables|Default|GetRootTurret) (Math|Rotator|MakeRotator 0.0 0.0 (.Yaw (Math|Rotator|BreakRotator (Math|Transform|InverseTransformRotation _returnvalue_2 (Math|Rotator|FindLookatRotation (Transformation|GetWorldLocation (Variables|Default|GetRootTurret)) _returnvalue_4))))) false false)
        (Transformation|SetRelativeRotation (Variables|Default|GetRootBurrel) (Math|Rotator|MakeRotator 0.0 (.Pitch (Math|Rotator|BreakRotator (Math|Transform|InverseTransformRotation _returnvalue_2 (Math|Rotator|FindLookatRotation (Transformation|GetWorldLocation (Variables|Default|GetRootBurrel)) _returnvalue_4)))) 0.0) false false)))
    (else
      (Transformation|AddRelativeRotation (Variables|Default|GetRootTurret) "0.0,1.000000,0.0" false false))))

(fn ConstructionScript)

(fn Fire
  (bind _arrowdirection (Variables|Default|GetArrowDirection))
  (bind _arrowdirection1 (Variables|Default|GetArrowDirection1))
  (bind _returnvalue (Transformation|GetWorldTransform _arrowdirection))
  (bind _returnvalue_2 (Transformation|GetWorldTransform _arrowdirection1))
  (Utilities|FlowControl|Sequence
    (:then_0
      (bind _returnvalue_3 (Game|SpawnActorfromClass "/Game/-RLS_Project/Enemies/Humanoid/Weapons/Projectiles/BP_Projectile_EnemyBulletTurret.BP_Projectile_EnemyBulletTurret_C" (Math|Transform|MakeTransform (.location _returnvalue) (.rotation _returnvalue) "1,1,1") "Undefined" 0 0))
      (Variables|/Game/-RLS_Project/Weapons/Projectiles/BP_Projectile_Base.BP_Projectile_Base_C|SetDamage _returnvalue_3 (Variables|Default|GetTurretDamage))
      (Variables|/Game/-RLS_Project/Weapons/Projectiles/BP_Projectile_Base.BP_Projectile_Base_C|SetDamageType _returnvalue_3 0)
      (Components|Activation|Activate (Variables|Default|GetMuzzle) true))
    (:then_1
      (bind _returnvalue_4 (Game|SpawnActorfromClass "/Game/-RLS_Project/Enemies/Humanoid/Weapons/Projectiles/BP_Projectile_EnemyBulletTurret.BP_Projectile_EnemyBulletTurret_C" (Math|Transform|MakeTransform (.location _returnvalue_2) (.rotation _returnvalue_2) "1,1,1") "Undefined" 0 0))
      (Variables|/Game/-RLS_Project/Weapons/Projectiles/BP_Projectile_Base.BP_Projectile_Base_C|SetDamage _returnvalue_4 (Variables|Default|GetTurretDamage))
      (Variables|/Game/-RLS_Project/Weapons/Projectiles/BP_Projectile_Base.BP_Projectile_Base_C|SetDamageType _returnvalue_4 0)
      (Components|Activation|Activate (Variables|Default|GetMuzzle1) true))))

(fn Raycast
  (Variables|Default|SetIsBlockingHit true)
  (Utilities|FlowControl|Sequence
    (:then_0
      (bind _outhit (Collision|SphereTraceByChannel (Transformation|GetWorldLocation (Variables|Default|GetArrowDirection)) (- (Camera|GetCameraLocation (Game|GetPlayerCameraManager 0)) "0, 0,20.000000") 5.0 "TraceTypeQuery1" false 0 "None" true "(R=1.000000,G=0.887261,B=0.000000,A=1.000000)" "(R=0.000000,G=1.000000,B=0.000000,A=1.000000)" 1.0))
      (Variables|Default|SetIsBlockingHit (.bBlockingHit (Collision|BreakHitResult _outhit))))
    (:then_1
      (bind _outhit_2 (Collision|SphereTraceByChannel (Transformation|GetWorldLocation (Variables|Default|GetArrowDirection1)) (- (Camera|GetCameraLocation (Game|GetPlayerCameraManager 0)) "0, 0,20.000000") 5.0 "TraceTypeQuery1" false 0 "None" true "(R=1.000000,G=0.887261,B=0.000000,A=1.000000)" "(R=0.000000,G=1.000000,B=0.000000,A=1.000000)" 1.0))
      (Variables|Default|SetIsBlockingHit (.bBlockingHit (Collision|BreakHitResult _outhit_2))))
    (:then_2
      (return (Variables|Default|GetIsBlockingHit)))))