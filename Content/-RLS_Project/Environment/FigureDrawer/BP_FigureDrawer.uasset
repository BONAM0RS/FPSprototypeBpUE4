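; BP_FigureDrawer draws debug-line stars, squares and cubes from functions, with an empty BeginPlay.
; DrawStar and DrawSquare step along a direction vector, rotating it about Z after each edge, using global color, duration, thickness and side length.
; DrawCube calls DrawSquare twice, offset perpendicular to the direction, and links the returned corners.
; DrawSquare ignores its SideLength input, so only the cube's offset honors it.
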(event EventBeginPlay)

(fn ConstructionScript)

(fn DrawStar
  (for _index (range 0 4)
    (Rendering|Debug|DrawDebugLine (LocalVariables|GetLocal_StartPoint) (+ (LocalVariables|GetLocal_StartPoint) (* (LocalVariables|GetLocal_Direction) (Variables|Default|GetGlobal_SideLength))) (Variables|Default|GetGlobal_DrawColor) (Variables|Default|GetGlobal_DrawDuration) (Variables|Default|GetGlobal_DrawThickness))
    (LocalVariables|SetLocal_StartPoint (+ (LocalVariables|GetLocal_StartPoint) (* (LocalVariables|GetLocal_Direction) (Variables|Default|GetGlobal_SideLength))))
    (LocalVariables|SetLocal_Direction (Math|Vector|RotateVectorAroundAxis (LocalVariables|GetLocal_Direction) 144.0 "0, 0,1.000000"))))

(fn DrawSquare
  (params (StartPoint :type Vector :default "140.000000,250.000000,100.000000") (Direction :type Vector :default "1.000000,0.000000,0") (SideLength :type Float%20%28single-precision%29))
  (LocalVariables|SetLocal_StartPoint StartPoint)
  (LocalVariables|SetLocal_Direction Direction)
  (Utilities|FlowControl|Sequence
    (:then_0
      (for _index (range 0 3)
        (Rendering|Debug|DrawDebugLine (LocalVariables|GetLocal_StartPoint) (+ (LocalVariables|GetLocal_StartPoint) (* (LocalVariables|GetLocal_Direction) (Variables|Default|GetGlobal_SideLength))) (Variables|Default|GetGlobal_DrawColor) (Variables|Default|GetGlobal_DrawDuration) (Variables|Default|GetGlobal_DrawThickness))
        (bind _output_get (LocalVariables|SetLocal_StartPoint (+ (LocalVariables|GetLocal_StartPoint) (* (LocalVariables|GetLocal_Direction) (Variables|Default|GetGlobal_SideLength)))))
        (Utilities|Array|Add (LocalVariables|GetLocal_SquarePoints) _output_get)
        (LocalVariables|SetLocal_Direction (Math|Vector|RotateVectorAroundAxis (LocalVariables|GetLocal_Direction) 9e+01 "0, 0,1.000000"))))
    (:then_1
      (return (LocalVariables|GetLocal_SquarePoints)))))

(fn DrawCube
  (params (StartPoint :type Vector :default "140.000000,400.000000,100.000000") (Direction :type Vector :default "1.000000,0.000000,0") (SideLength :type Float%20%28single-precision%29))
  (Utilities|FlowControl|Sequence
    (:then_0
      (bind _squarepoints (CallFunction|DrawSquare StartPoint Direction SideLength))
      (LocalVariables|SetLocal_StartPoints _squarepoints))
    (:then_1
      (bind _squarepoints_2 (CallFunction|DrawSquare (+ StartPoint (* (Math|Vector|RotateVectorAroundAxis Direction -9e+01 "0.000000,1.000000, 0") SideLength)) Direction SideLength))
      (LocalVariables|SetLocal_EndPoints _squarepoints_2))
    (:then_2
      (for (_array_element _array_index) (LocalVariables|GetLocal_StartPoints)
        (Rendering|Debug|DrawDebugLine _array_element (Utilities|Array|Get(acopy) (LocalVariables|GetLocal_EndPoints) _array_index) (Variables|Default|GetGlobal_DrawColor) (Variables|Default|GetGlobal_DrawDuration) (Variables|Default|GetGlobal_DrawThickness))))))