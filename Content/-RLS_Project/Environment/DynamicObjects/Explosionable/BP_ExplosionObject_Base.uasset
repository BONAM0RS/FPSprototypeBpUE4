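; BP_ExplosionObject_Base is a base explosive prop that detonates from hard impacts or damage.
; A hit above the impulse threshold explodes it immediately, the first HP change ignites fire and explodes it after a random delay, and death explodes it after a short delay.
; All triggers share a DoOnce-guarded Explode that spawns effects, sound and camera shake, applies radial falloff damage, then destroys the actor.
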(event OnComponentHit(ObjectMesh)
  (params (HitComponent :type Primitive%20Component%20Object%20Reference) (OtherActor :type Actor%20Object%20Reference) (OtherComp :type Primitive%20Component%20Object%20Reference) (NormalImpulse :type Vector :default "0, 0, 0") (Hit :type Hit%20Result%20Structure%20%28by%20ref%29))
  (if (> (Math|Vector|VectorLength NormalImpulse) (Variables|-Damage|GetImpulse))
    (CallFunction|Explode)))

(event OnChangedHP(BP_VitalityComponent)
  (params (CurrentHP :type Float%20%28single-precision%29) (TotalHP :type Float%20%28single-precision%29))
  (if (not (Variables|Default|GetIsFire))
    (Variables|Default|SetIsFire true)
    (Components|Activation|Activate (Variables|Default|GetParticleSystem_Fire) true)
    (Utilities|FlowControl|Delay (Math|Random|RandomFloatinRange 2.0 5.0))
    (CallFunction|Explode)))

(event OnDied(BP_VitalityComponent)
  (Utilities|FlowControl|Delay 1.0)
  (CallFunction|Explode))

(event Custom|Explode
  (bind _returnvalue (Transformation|GetActorLocation))
  (bind _damage (Variables|-Damage|GetDamage))
  (bind _radius (Variables|-Damage|GetRadius))
  (bind _radius_2 (Variables|-Damage|GetRadius))
  (Utilities|FlowControl|DoOnce false
    (:Completed
      (Utilities|FlowControl|Sequence
        (:then_0
          (Effects|SpawnEmitteratLocation "/Game/MilitaryWeapDark/FX/P_Grenade_Explosion_01.P_Grenade_Explosion_01" _returnvalue)
          (Audio|SpawnSoundatLocation "/Game/MilitaryWeapDark/Sound/GrenadeLauncher/GrenadeLauncher_Explosion_Cue.GrenadeLauncher_Explosion_Cue" _returnvalue "0, 0, 0" 0.1 1.0 0.0 0 0)
          (Camera|PlayWorldCameraShake "/Game/-RLS_Project/Weapons/Projectiles/BP_Explosion_CamShake_Matinee.BP_Explosion_CamShake_Matinee_C" _returnvalue (/ _radius 3.0) _radius 1.0 true))
        (:then_1
          (Class|GameplayStatics|ApplyRadialDamagewithFalloff _damage (/ _damage 5.0) (Transformation|GetActorLocation) (/ _radius_2 3.0) _radius_2 1.0 (Variables|Default|GetExplosionDamageType) 0 0 0 "ECC_GameTraceChannel3"))
        (:then_2
          (Actor|DestroyActor))))))

(fn ConstructionScript)