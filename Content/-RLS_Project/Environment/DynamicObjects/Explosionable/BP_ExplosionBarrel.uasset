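; BP_ExplosionBarrel is an interactable barrel that shows an on-screen prompt when focused.
; OnFocus lazily caches the UI widget from the player's BP_Hero, then shows or hides its interact text, choosing focus or interacted wording based on IsGrab.
; Grab sets IsGrab and switches the prompt to the interacted text.
; GetInfo returns an empty string, and no explosion logic appears in these graphs.
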(event EventBeginPlay)

(event Collision|EventActorBeginOverlap
  (params (OtherActor :type Actor%20Object%20Reference)))

(event EventTick
  (params (DeltaSeconds :type Float%20%28single-precision%29)))

(event EventOnFocus
  (params (OnOff :type Boolean))
  (Utilities|IsValid (Variables|Default|GetWBP_UI)
    (:Is%20Valid
      _)
    (:Is%20Not%20Valid
      (bind _asbp_hero (Utilities|Casting|CastToBP_Hero (Game|GetPlayerCharacter 0)))
      (Variables|Default|SetWBP_UI (Variables|/Game/-RLS_Project/Hero/BP_Hero.BP_Hero_C|GetUI _asbp_hero))))
  (if OnOff
    (if (Variables|Default|GetIsGrab)
      (Default|SetInteractText (Variables|Default|GetWBP_UI) (Variables|Default|GetInteractedText))
      (else
        (Default|SetInteractText (Variables|Default|GetWBP_UI) (Variables|Default|GetFocusText))))
    (Widget|SetVisibility (Variables|/Game/-RLS_Project/UI/Widgets/WBP_UI.WBP_UI_C|GetText_Interact (Variables|Default|GetWBP_UI)) "Visible")
    (else
      (Widget|SetVisibility (Variables|/Game/-RLS_Project/UI/Widgets/WBP_UI.WBP_UI_C|GetText_Interact (Variables|Default|GetWBP_UI)) "Collapsed"))))

(event EventGrab
  (Variables|Default|SetIsGrab true)
  (Default|SetInteractText (Variables|Default|GetWBP_UI) (Variables|Default|GetInteractedText)))

(fn ConstructionScript
  (|CallParentFunction))

(fn GetInfo
  (return ""))