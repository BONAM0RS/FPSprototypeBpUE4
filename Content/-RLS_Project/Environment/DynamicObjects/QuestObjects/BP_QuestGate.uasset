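; BP_QuestGate is a quest environment gate that opens by sliding along its Z axis when OpenGate is called.
; A timeline, with play rate scaled by OpenDuration, lerps SlidingRoot's relative height from zero to Height.
; Opening also triggers ChangeColor, which turns the point light green, swaps the exit table material, and hides the light some seconds after the opening duration ends.
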(event Custom|OpenGate
  (CallFunction|ChangeColor)
  (Development|PrintString "Open Gate!")
  (Components|Timeline|SetPlayRate (Variables|Default|GetGate_TimeLine) (/ 1.0 (Variables|Default|GetOpenDuration)))
  (bind _gate (Timeline|Gate_Timeline Play)
    (:Update
      (Transformation|SetRelativeLocation (Variables|Default|GetSlidingRoot) (Math|Vector|MakeVector 0.0 0.0 (Math|Float|Lerp 0.0 (Variables|Default|GetHeight) _gate)) false false))))

(event Custom|ChangeColor
  (Rendering|Components|Light|SetLightColor (Variables|Default|GetPointLight) "(R=0.000000,G=1.000000,B=0.181207,A=1.000000)" true)
  (Rendering|Material|SetMaterial (Variables|Default|GetExitTable) 0 "/Game/StorageHouse/Materials/M_Exit_02.M_Exit_02")
  (Utilities|FlowControl|Delay (+ (Variables|Default|GetOpenDuration) 1e+01))
  (Rendering|SetVisibility (Variables|Default|GetPointLight) false false))

(fn ConstructionScript)