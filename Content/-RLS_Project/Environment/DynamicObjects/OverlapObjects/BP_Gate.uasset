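; BP_Gate is an environment gate that slides vertically when a character overlaps its Activator and can be destroyed.
; Overlap begin and end events play or reverse a timeline that lerps GateRoot's relative Z up to Height, with play rate derived from OpenDuration or CloseDuration.
; When its vitality component fires OnDied, the Gate component is destroyed.
; The setup excluding cube components from damage is unconnected and never runs.
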(event OnDied(BP_VitalityComponent)
  (bind _gate (Variables|Default|GetGate))
  (Utilities|IsValid _gate
    (:Is%20Valid
      (Components|DestroyComponent _gate))))

(event Custom|On%20Begin%20Overlap
  (params (Character :type Actor%20Object%20Reference))
  (Development|PrintString "Begin")
  (Components|Timeline|SetPlayRate (Variables|Default|GetGate_TimeLine) (/ 1.0 (Variables|Default|GetOpenDuration)))
  (bind _gate (Timeline|Gate_TimeLine Play)
    (:Update
      (Transformation|SetRelativeLocation (Variables|Default|GetGateRoot) (Math|Vector|MakeVector 0.0 0.0 (Math|Float|Lerp 0.0 (Variables|Default|GetHeight) _gate)) false false))))

(event Custom|On%20End%20Overlap
  (params (Character :type Actor%20Object%20Reference))
  (Development|PrintString "End")
  (Components|Timeline|SetPlayRate (Variables|Default|GetGate_TimeLine) (/ 1.0 (Variables|Default|GetCloseDuration)))
  (bind _gate (Timeline|Gate_TimeLine Reverse)
    (:Update
      (Transformation|SetRelativeLocation (Variables|Default|GetGateRoot) (Math|Vector|MakeVector 0.0 0.0 (Math|Float|Lerp 0.0 (Variables|Default|GetHeight) _gate)) false false))))

(event EventBeginPlay
  (EventDispatchers|BindEventtoOnCharacterBeginOverlap (Variables|Default|GetActivator) (delegate Custom|On%20Begin%20Overlap))
  (EventDispatchers|BindEventtoOnCharacterEndOverlap (Variables|Default|GetActivator) (EventDispatchers|CreateEvent :!event Custom|On%20End%20Overlap)))

(fn ConstructionScript)