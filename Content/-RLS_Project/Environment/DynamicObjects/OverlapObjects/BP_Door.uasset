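; BP_Door is a door that swings open when a character overlaps its Activator and closes when the overlap ends.
; BeginPlay binds to the Activator's character overlap events and sets the timeline play rate from Duration.
; The overlap events play or reverse the timeline, whose curve lerps DoorRoot's relative yaw between zero and Rotation, printing debug strings on begin and end.
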(event Custom|On%20Begin%20Overlap
  (params (Character :type Actor%20Object%20Reference))
  (Development|PrintString "Begin")
  (bind _door (Timeline|Door_TimeLine Play)
    (:Update
      (Transformation|SetRelativeRotation (Variables|Default|GetDoorRoot) (Math|Rotator|MakeRotator 0.0 0.0 (Math|Float|Lerp 0.0 (Variables|Default|GetRotation) _door)) false false))))

(event Custom|On%20End%20Overlap
  (params (Character :type Actor%20Object%20Reference))
  (Development|PrintString "End")
  (bind _door (Timeline|Door_TimeLine Reverse)
    (:Update
      (Transformation|SetRelativeRotation (Variables|Default|GetDoorRoot) (Math|Rotator|MakeRotator 0.0 0.0 (Math|Float|Lerp 0.0 (Variables|Default|GetRotation) _door)) false false))))

(event EventBeginPlay
  (bind _activator (Variables|Default|GetActivator))
  (EventDispatchers|BindEventtoOnCharacterBeginOverlap _activator (delegate Custom|On%20Begin%20Overlap))
  (EventDispatchers|BindEventtoOnCharacterEndOverlap _activator (EventDispatchers|CreateEvent :!event Custom|On%20End%20Overlap))
  (Components|Timeline|SetPlayRate (Variables|Default|GetDoor_TimeLine) (/ 1.0 (Variables|Default|GetDuration))))

(fn ConstructionScript)