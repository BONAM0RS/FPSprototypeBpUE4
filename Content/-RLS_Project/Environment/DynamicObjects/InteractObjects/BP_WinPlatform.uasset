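; Elevator-style win platform that shows the win screen and starts moving the first time an actor tagged Character enters its collision box.
; BeginPlay creates the win widget, sets timeline speed from MoveTime and binds to the button events of linked InteractActivators.
; OnButton flip-flops the timeline between play and reverse, lerping the Scene component with sweep from its start location to an EndLocation offset.
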(event OnComponentBeginOverlap(CollisionBox)
  (params (OverlappedComponent :type Primitive%20Component%20Object%20Reference) (OtherActor :type Actor%20Object%20Reference) (OtherComp :type Primitive%20Component%20Object%20Reference) (OtherBodyIndex :type Integer) (bFromSweep :type Boolean) (SweepResult :type Hit%20Result%20Structure%20%28by%20ref%29))
  (if (not (Variables|Default|GetIsWin))
    (if (Actor|ActorHasTag OtherActor "Character")
      (Default|ShowWinScreen (Variables|Default|GetUI_WinScreen))
      (Variables|Default|SetIsWin true)
      (CallFunction|OnButton))))

(event Custom|OnButton
  (bind _startlocation (Variables|Default|GetStartLocation))
  (Utilities|FlowControl|FlipFlop
    (:A
      (bind _elevatortrack (Timeline|Elevator_Timeline Play)
        (:Update
          (Transformation|SetRelativeLocation (Variables|Default|GetScene) (Math|Vector|Lerp(Vector) _startlocation (+ _startlocation (Variables|Default|GetEndLocation)) _elevatortrack) true false))))
    (:B
      (Timeline|Elevator_Timeline Reverse))))

(event Collision|EventActorBeginOverlap
  (params (OtherActor :type Actor%20Object%20Reference)))

(event EventBeginPlay
  (bind _returnvalue (UserInterface|CreateWidget "/Game/-RLS_Project/UI/Widgets/WBP_WinScreen.WBP_WinScreen_C"))
  (Variables|Default|SetUI_WinScreen _returnvalue)
  (Variables|Default|SetStartLocation (Transformation|GetActorLocation))
  (Components|Timeline|SetPlayRate (Variables|Default|GetElevator_Timeline) (/ 1.0 (Variables|Default|GetMoveTime)))
  (for _array_element (Variables|Default|GetInteract_Activators)
    (EventDispatchers|BindEventtoOnButton _array_element (EventDispatchers|CreateEvent :!event Custom|OnButton))))

(fn ConstructionScript)