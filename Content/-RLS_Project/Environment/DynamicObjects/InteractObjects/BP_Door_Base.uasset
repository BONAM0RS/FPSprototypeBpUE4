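; BP_Door_Base is an interactable door that swings open and closed in response to linked InteractActivators.
; On BeginPlay it binds to each activator's button and lever events: buttons toggle the door, while levers set it to match their state.
; A timeline plays or reverses to rotate DoorRoot's yaw up to RotateAngle, flipping IsOpen when finished.
; The Construction Script adds a curved spline from the door to each activator, visualizing the links.
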(event Custom|OnLever
  (params (IsActive :type Boolean))
  (bind _isopen (Variables|Default|GetIsOpen))
  (if IsActive
    (if (not _isopen)
      (CallFunction|Open))
    (elif _isopen
      (CallFunction|Close))))

(event Custom|OnButton
  (if (not (Variables|Default|GetIsOpen))
    (CallFunction|Open)
    (else
      (CallFunction|Close))))

(event Custom|Open
  (bind _opentrack (Timeline|Open_Timeline Play)
    (:Update
      (Transformation|SetRelativeRotation (Variables|Default|GetDoorRoot) (Math|Rotator|MakeRotator 0.0 0.0 (Math|Float|Lerp 0.0 (Variables|Default|GetRotateAngle) _opentrack)) false false))
    (:Finished
      (Variables|Default|SetIsOpen (not (Variables|Default|GetIsOpen))))))

(event Custom|Close
  (bind _opentrack (Timeline|Open_Timeline Reverse)
    (:Update
      (Transformation|SetRelativeRotation (Variables|Default|GetDoorRoot) (Math|Rotator|MakeRotator 0.0 0.0 (Math|Float|Lerp 0.0 (Variables|Default|GetRotateAngle) _opentrack)) false false))
    (:Finished
      (Variables|Default|SetIsOpen (not (Variables|Default|GetIsOpen))))))

(event EventBeginPlay
  (for _array_element (Variables|Default|GetInteractActivators)
    (EventDispatchers|BindEventtoOnLever _array_element (EventDispatchers|CreateEvent :!event Custom|OnLever))
    (EventDispatchers|BindEventtoOnButton _array_element (EventDispatchers|CreateEvent :!event Custom|OnButton))))

(fn ConstructionScript
  (for _array_element (Variables|Default|GetInteractActivators)
    (bind _returnvalue (AddComponent|AddSplineComponent false))
    (Spline|SetLocationatSplinePoint _returnvalue 1 (.Origin (Collision|GetActorBounds _array_element true false)) "World" true)
    (Spline|SetLocationatSplinePoint _returnvalue 0 (.Origin (Collision|GetActorBounds true false)) "World" true)
    (Spline|SetTangentatSplinePoint _returnvalue 1 (Math|Vector|MakeVector 0.0 0.0 -3e+02) "Local" true)))