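; BP_Elevator_Base is a base elevator that travels between its starting point and an EndLocation offset when linked activators fire.
; On BeginPlay it caches its location, scales the timeline play rate by MoveTime, and binds to each InteractActivator's button event.
; Each press alternately plays or reverses the timeline, lerping ElevatorRoot with sweep.
; The cached world location feeds a relative-location setter.
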(event Custom|OnButton
  (bind _startlocation (Variables|Default|GetStartLocation))
  (Utilities|FlowControl|FlipFlop
    (:A
      (bind _elevatortrack (Timeline|Elevator_Timeline Play)
        (:Update
          (Transformation|SetRelativeLocation (Variables|Default|GetElevatorRoot) (Math|Vector|Lerp(Vector) _startlocation (+ _startlocation (Variables|Default|GetEndLocation)) _elevatortrack) true false))))
    (:B
      (Timeline|Elevator_Timeline Reverse))))

(event EventBeginPlay
  (Variables|Default|SetStartLocation (Transformation|GetActorLocation))
  (Components|Timeline|SetPlayRate (Variables|Default|GetElevator_Timeline) (/ 1.0 (Variables|Default|GetMoveTime)))
  (for _array_element (Variables|Default|GetInteractActivators)
    (EventDispatchers|BindEventtoOnButton _array_element (EventDispatchers|CreateEvent :!event Custom|OnButton))))

(fn ConstructionScript)