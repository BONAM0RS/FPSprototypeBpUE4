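; Interactable standard door that swings open and shut when the player interacts with it.
; On focus it shows or hides an interact prompt in the hero's UI, caching that widget from BP_Hero when needed.
; Interact plays or reverses a timeline that lerps the door root's yaw between zero and a set angle.
; The open state flips only when the timeline finishes, and GetInfo returns an empty string.
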(event EventOnFocus
  (params (OnOff :type Boolean))
  (Utilities|IsValid (Variables|Default|GetWBP_UI)
    (:Is%20Valid
      _)
    (:Is%20Not%20Valid
      (bind _asbp_hero (Utilities|Casting|CastToBP_Hero (Game|GetPlayerCharacter 0)))
      (Variables|Default|SetWBP_UI (Variables|/Game/-RLS_Project/Hero/BP_Hero.BP_Hero_C|GetUI _asbp_hero))))
  (if OnOff
    (Default|SetInteractText (Variables|Default|GetWBP_UI) (Variables|Default|GetFocusText))
    (Widget|SetVisibility (Variables|/Game/-RLS_Project/UI/Widgets/WBP_UI.WBP_UI_C|GetText_Interact (Variables|Default|GetWBP_UI)) "Visible")
    (else
      (Widget|SetVisibility (Variables|/Game/-RLS_Project/UI/Widgets/WBP_UI.WBP_UI_C|GetText_Interact (Variables|Default|GetWBP_UI)) "Collapsed"))))

(event EventInteract
  (if (not (Variables|Default|GetIsOpen))
    (bind _opentrack (Timeline|Open_Timeline Play)
      (:Update
        (Transformation|SetRelativeRotation (Variables|Default|GetRootDoor) (Math|Rotator|MakeRotator 0.0 0.0 (Math|Float|Lerp 0.0 (Variables|Default|GetRotateAngle) _opentrack)) false false))
      (:Finished
        (Variables|Default|SetIsOpen (not (Variables|Default|GetIsOpen)))))
    (else
      (Timeline|Open_Timeline Reverse))))

(fn ConstructionScript)

(fn GetInfo
  (return ""))