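; BP_ImpactEffect is a short-lived actor that plays impact effects at the point described by its HitResult.
; On BeginPlay, if the hit has a valid physical material, it picks a particle emitter by surface type (wood, metal, water, asphalt default).
; It also spawns a temporary fabric decal aligned to the impact normal, whatever the surface, then destroys itself.
; The SpawnImpactEffect event is empty.
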(event Custom|SpawnImpactEffect
  (params (HitResult :type Hit%20Result%20Structure)))

(event EventBeginPlay
  (bind _hitresult (Variables|Default|GetHitResult))
  (bind (_bblockinghit _binitialoverlap _time _distance _location _impactpoint _normal _impactnormal _physmat) (Collision|BreakHitResult _hitresult))
  (Utilities|FlowControl|Sequence
    (:then_0
      (Utilities|IsValid _physmat
        (:Is%20Valid
          (Effects|SpawnEmitteratLocation (Utilities|Select :Index (Variables|/Script/PhysicsCore.PhysicalMaterial|GetSurfaceType _physmat) :SurfaceType_Default "/Game/BallisticsVFX/Particles/Impacts/DynamicImpacts/Asphalt/Asphalt_impact_Dyn.Asphalt_impact_Dyn" :SurfaceType1 "/Game/BallisticsVFX/Particles/Impacts/DynamicImpacts/Wood/Wood_impact_Dyn.Wood_impact_Dyn" :SurfaceType2 "/Game/BallisticsVFX/Particles/Impacts/DynamicImpacts/Metal/Metal_impact_Dyn.Metal_impact_Dyn" :SurfaceType3 "/Game/BallisticsVFX/Particles/Impacts/DynamicImpacts/Water/Water_impact_Dyn.Water_impact_Dyn") _impactpoint)
          (bind _returnvalue (Rendering|Decal|SpawnDecalatLocation "/Game/BallisticsVFX/Decals/Decals_Fabric.Decals_Fabric" "2.000000,4.000000,4.000000" _impactpoint (Math|Conversions|RotationFromXVector _impactnormal) 1e+01))
          (Rendering|Components|Decal|SetFadeScreenSize _returnvalue 0.001))))
    (:then_1
      (Actor|DestroyActor))))

(fn ConstructionScript)