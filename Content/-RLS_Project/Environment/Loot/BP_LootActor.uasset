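; Data-table-driven loot pickup that the player focuses and interacts with to gain an effect.
; BeginPlay reads its row to async-load the mesh, set scale and tint the light, then self-destroys DestroyDelay after the mesh loads.
; Focus toggles a named pickup prompt on the hero's UI.
; Interact async-loads the row's effect class, constructs a BP_LootEffect_Base object to apply it to the hero, then destroys the actor.
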(event EventBeginPlay
  (bind _content (Variables|Default|GetContent))
  (bind (_datatable _rowname) (Utilities|Struct|BreakDataTableRowHandle _content))
  (bind _returnvalue (Utilities|GetDataTableRow _datatable _rowname)
    (:then
      (bind _output_get (Variables|Default|SetStructContent _returnvalue))
      (bind _asbp_hero (Utilities|Casting|CastToBP_Hero (Game|GetPlayerCharacter 0)))
      (Variables|Default|SetWBP_UI (Variables|/Game/-RLS_Project/Hero/BP_Hero.BP_Hero_C|GetUI _asbp_hero))
      (Utilities|FlowControl|Sequence
        (:then_0
          (bind _object (Utilities|AsyncLoadAsset (.Mesh (Utilities|Struct|BreakStruct_LootParams _output_get)))
            (:Completed
              (bind _asstatic_mesh (Utilities|Casting|CastToStaticMesh _object))
              (Components|StaticMesh|SetStaticMesh (Variables|Default|GetLootMesh) _asstatic_mesh)
              (Utilities|FlowControl|Delay (Variables|Default|GetDestroyDelay))
              (Actor|DestroyActor))))
        (:then_1
          (Rendering|Components|Light|SetLightColor (Variables|Default|GetPointLight) (.NameColor (Utilities|Struct|BreakStruct_LootParams _output_get)) true)
          (Transformation|SetWorldScale3D (Variables|Default|GetLootMesh) (.Scale (Utilities|Struct|BreakStruct_LootParams _output_get))))))))

(event EventInteract
  (bind _class (Utilities|AsyncLoadClassAsset (.LootEffect (Utilities|Struct|BreakStruct_LootParams (Variables|Default|GetStructContent))))
    (:Completed
      (bind _asbp_loot_effect_base (Utilities|Casting|CastToBP_LootEffect_BaseClass _class))
      (bind _returnvalue (Game|ConstructObjectfromClass _asbp_loot_effect_base self))
      (Default|ApplyEffecttoHero _returnvalue (.AsBP%20Hero (Utilities|Casting|CastToBP_Hero (Game|GetPlayerCharacter 0))) (Variables|Default|GetStructContent))
      (Widget|SetVisibility (Variables|/Game/-RLS_Project/UI/Widgets/WBP_UI.WBP_UI_C|GetText_Interact (Variables|Default|GetWBP_UI)) "Hidden")
      (Actor|DestroyActor))))

(event EventOnFocus
  (params (OnOff :type Boolean))
  (if OnOff
    (Default|SetInteractText (Variables|Default|GetWBP_UI) (Utilities|String|StringToName (Utilities|String|Append "[ F ] Pick up: " (.Name (Utilities|Struct|BreakStruct_LootParams (Variables|Default|GetStructContent))))))
    (Widget|SetVisibility (Variables|/Game/-RLS_Project/UI/Widgets/WBP_UI.WBP_UI_C|GetText_Interact (Variables|Default|GetWBP_UI)) "Visible")
    (else
      (Widget|SetVisibility (Variables|/Game/-RLS_Project/UI/Widgets/WBP_UI.WBP_UI_C|GetText_Interact (Variables|Default|GetWBP_UI)) "Collapsed"))))

(fn ConstructionScript)

(fn GetInfo
  (return ""))