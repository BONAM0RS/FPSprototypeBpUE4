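; BP_LootEffect_Ammo_Base is a base loot effect that grants ammo to a hero's weapons.
; Its ApplyEffectToHero override runs the parent logic, then loops over the hero's Weapons.
; Each weapon whose WeaponChoose matches the effect's own receives the effect's Amount through AddAmmo, with IsMain passed along.
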(fn ApplyEffecttoHero
  (params (Hero :type BP%20Hero%20Object%20Reference) (Effect :type Struct%20Loot%20Params%20Structure))
  (|CallParentFunction Hero Effect)
  (for _array_element (Variables|/Game/-RLS_Project/Hero/BP_Hero.BP_Hero_C|GetWeapons Hero)
    (if (== (Variables|/Game/-RLS_Project/Weapons/BP_Weapon_Base.BP_Weapon_Base_C|GetWeaponChoose _array_element) (Variables|Default|GetWeaponChoose))
      (Default|AddAmmo _array_element (.Amount (Utilities|Struct|BreakStruct_LootParams Effect)) (Variables|Default|GetIsMain) (Variables|/Game/-RLS_Project/Weapons/BP_Weapon_Base.BP_Weapon_Base_C|GetWeaponChoose _array_element)))))