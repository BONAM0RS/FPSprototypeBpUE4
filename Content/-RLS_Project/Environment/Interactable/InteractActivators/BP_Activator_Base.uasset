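; BP_Activator_Base is, by name and folder, the base Blueprint for interactable activators.
; It exposes an OnFocus event with no logic and a GetInfo function that returns an empty string.
; An unwired leftover graph would cache the BP_Hero UI widget, then show FocusText as the interact prompt or collapse it, but it never runs.
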(event EventOnFocus
  (params (OnOff :type Boolean)))

(fn ConstructionScript)

(fn GetInfo
  (return ""))