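; Base lever interactable that players toggle between two states, highlighted by a point light while focused.
; Interact plays or reverses a timeline that pitches the handle between the absolute and signed MoveAngle, ignoring input while it moves.
; When the swing finishes, it flips IsActive and broadcasts the new state through the OnLever dispatcher.
; GetInfo supplies the lever's interaction display data.
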(event EventOnFocus
  (params (OnOff :type Boolean))
  (Rendering|SetVisibility (Variables|Default|GetPointLight) OnOff false))

(event EventInteract
  (bind _moveangle (Variables|-InteractSettings|GetMoveAngle))
  (if (not (Variables|-InteractSettings|GetIsMove))
    (Variables|-InteractSettings|SetIsMove true)
    (if (not (Variables|-InteractSettings|GetIsActive))
      (bind _levertrack (Timeline|MoveLever_Timeline Play)
        (:Update
          (Transformation|SetRelativeRotation (Variables|Default|GetHandleRoot) (Math|Rotator|MakeRotator 0.0 (Math|Float|Lerp (Math|Float|Absolute(Float) _moveangle) _moveangle _levertrack) 0.0) false false))
        (:Finished
          (bind _output_get (Variables|-InteractSettings|SetIsActive (not (Variables|-InteractSettings|GetIsActive))))
          (Variables|-InteractSettings|SetIsMove false)
          (Default|CallOnLever _output_get)))
      (else
        (Timeline|MoveLever_Timeline Reverse)))))

(fn ConstructionScript
  (|CallParentFunction))

(fn GetInfo
  (return (Variables|-InteractSettings|GetInteractDisplay)))