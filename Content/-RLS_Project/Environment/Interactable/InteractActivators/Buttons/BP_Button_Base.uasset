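; BP_Button_Base is a base pushable button that the player can focus and interact with to trigger OnButton.
; Focus toggles a point light and a text prompt on the hero's UI widget, which is fetched from BP_Hero and cached when invalid.
; Interact plays a timeline that moves the button root along X, ignoring presses while moving; an event track fires OnButton during the motion.
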(event EventOnFocus
  (params (OnOff :type Boolean))
  (Rendering|SetVisibility (Variables|Default|GetPointLight) OnOff false)
  (Utilities|IsValid (Variables|Default|GetWBP_UI)
    (:Is%20Valid
      _)
    (:Is%20Not%20Valid
      (bind _asbp_hero (Utilities|Casting|CastToBP_Hero (Game|GetPlayerCharacter 0)))
      (Variables|Default|SetWBP_UI (Variables|/Game/-RLS_Project/Hero/BP_Hero.BP_Hero_C|GetUI _asbp_hero))))
  (if OnOff
    (Default|SetInteractText (Variables|Default|GetWBP_UI) (Variables|Default|GetFocusText))
    (Widget|SetVisibility (Variables|/Game/-RLS_Project/UI/Widgets/WBP_UI.WBP_UI_C|GetText_Interact (Variables|Default|GetWBP_UI)) "Visible")
    (else
      (Widget|SetVisibility (Variables|/Game/-RLS_Project/UI/Widgets/WBP_UI.WBP_UI_C|GetText_Interact (Variables|Default|GetWBP_UI)) "Collapsed"))))

(event EventInteract
  (if (not (Variables|-InteractSettings|GetIsMove))
    (Variables|-InteractSettings|SetIsMove true)
    (bind _buttontrack (Timeline|MoveButton_Timeline PlayFromStart)
      (:Update
        (Transformation|SetRelativeLocation (Variables|Default|GetButtonRoot) (Math|Vector|MakeVector (Math|Float|Lerp 0.0 (Variables|-InteractSettings|GetMoveDistance) _buttontrack) 0.0 0.0) false false))
      (:Finished
        (Variables|-InteractSettings|SetIsMove false))
      (:PushButtonEvent
        (Default|CallOnButton)))))

(fn ConstructionScript
  (|CallParentFunction))

(fn GetInfo
  (return (Variables|-InteractSettings|GetInteractDisplay)))