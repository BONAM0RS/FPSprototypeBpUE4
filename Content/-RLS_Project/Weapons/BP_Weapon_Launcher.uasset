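; Launcher weapon that fires rockets as its main shot and grenades as its alternate shot.
; TryMakeShot runs the parent check, then spends ammo (total pool for rockets, current alt count for grenades) and applies fire-rate control.
; A camera sphere trace sets the aim point, and the projectile spawns at that mode's muzzle component facing it.
; Projectiles receive damage from shot parameters; the DamageType assignments are disconnected.
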(event Custom|LaunchRocket
  (bind _returnvalue (Game|GetPlayerCameraManager 0))
  (bind _main_dir (Variables|Default|GetMain_Dir))
  (bind _returnvalue_2 (Transformation|GetWorldTransform _main_dir))
  (bind _returnvalue_3 (Camera|GetCameraLocation _returnvalue))
  (bind _result (CallFunction|TrySpendAmmo true))
  (if _result
    (CallFunction|FireRateControl true)
    (bind _outhit (Collision|SphereTraceByChannel _returnvalue_3 (+ _returnvalue_3 (* (Transformation|GetActorForwardVector _returnvalue) 3e+03)) 5.0 "TraceTypeQuery1" false 0 "None" true "(R=1.000000,G=0.000000,B=0.000000,A=1.000000)" "(R=0.000000,G=1.000000,B=0.000000,A=1.000000)" 1.0))
    (bind _returnvalue_4 (Game|SpawnActorfromClass "/Game/-RLS_Project/Weapons/Projectiles/BP_Projectile_Rocket.BP_Projectile_Rocket_C" (Math|Transform|MakeTransform (.location _returnvalue_2) (Math|Rotator|FindLookatRotation (.location _returnvalue_2) (select (.bBlockingHit (Collision|BreakHitResult _outhit)) (.ImpactPoint (Collision|BreakHitResult _outhit)) (.TraceEnd (Collision|BreakHitResult _outhit)))) "1,1,1") "Undefined" 0 0))
    (Variables|/Game/-RLS_Project/Weapons/Projectiles/BP_Projectile_Base.BP_Projectile_Base_C|SetDamage _returnvalue_4 (.Damage (Utilities|Struct|BreakStruct_WeaponShotParam (Variables|Default|GetMainShotParam))))))

(event Custom|LaunchGrenade
  (bind _returnvalue (Game|GetPlayerCameraManager 0))
  (bind _alt_dir (Variables|Default|GetAlt_Dir))
  (bind _returnvalue_2 (Camera|GetCameraLocation _returnvalue))
  (bind _returnvalue_3 (Transformation|GetWorldTransform _alt_dir))
  (bind _result (CallFunction|TrySpendAmmo false))
  (if _result
    (CallFunction|FireRateControl false)
    (bind _outhit (Collision|SphereTraceByChannel _returnvalue_2 (+ _returnvalue_2 (* (Transformation|GetActorForwardVector _returnvalue) 3e+03)) 5.0 "TraceTypeQuery1" false 0 "None" true "(R=1.000000,G=0.000000,B=0.000000,A=1.000000)" "(R=0.000000,G=1.000000,B=0.000000,A=1.000000)" 1.0))
    (bind _returnvalue_4 (Game|SpawnActorfromClass "/Game/-RLS_Project/Weapons/Projectiles/BP_Projectile_Grenade.BP_Projectile_Grenade_C" (Math|Transform|MakeTransform (.location _returnvalue_3) (Math|Rotator|FindLookatRotation (.location _returnvalue_3) (select (.bBlockingHit (Collision|BreakHitResult _outhit)) (.ImpactPoint (Collision|BreakHitResult _outhit)) (.TraceEnd (Collision|BreakHitResult _outhit)))) "1,1,1") "Undefined" 0 0))
    (Variables|/Game/-RLS_Project/Weapons/Projectiles/BP_Projectile_Base.BP_Projectile_Base_C|SetDamage _returnvalue_4 (.Damage (Utilities|Struct|BreakStruct_WeaponShotParam (Variables|Default|GetAltShotParam))))))

(fn ConstructionScript
  (|CallParentFunction))

(fn TryMakeShot
  (params (IsMain :type Boolean))
  (bind _result (|CallParentFunction false))
  (if _result
    (if IsMain
      (CallFunction|LaunchRocket)
      (else
        (CallFunction|LaunchGrenade)))))

(fn TrySpendAmmo
  (params (IsMain :type Boolean))
  (if (> (select IsMain (Variables|Default|GetTotalAmmo_Main) (Variables|Default|GetCurrentAmmo_Alt)) 0)
    (Math|Integer|DecrementInt (select IsMain (Variables|Default|GetTotalAmmo_Main) (Variables|Default|GetCurrentAmmo_Alt))
      (:%20%20
        (CallFunction|SendAmmoInfo)
        (Default|CallOnShot)
        (return true)))
    (else
      (return false))))