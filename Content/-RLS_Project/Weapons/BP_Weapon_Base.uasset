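; Base weapon Blueprint providing shared main and alternate fire logic, ammo handling and effects for the player's guns.
; Shots are camera-origin sphere traces with random cone scatter, spawning impact effects and applying point damage, doubled with critical text on "head" bone hits.
; A delay-gated IsFire flag limits fire rate per mode.
; Ammo functions handle spending, pickups and main-clip reloads, reporting through shot and ammo-change calls.
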(event Custom|WeaponStartReload
  (Animation|Montage|PlayMontage (Variables|Default|GetWeaponMesh) (Variables|-Montages|GetWeaponReloadMontage)))

(event Custom|FireRateControl
  (params (IsMain :type Boolean))
  (if IsMain
    (Variables|Default|SetIsFire false)
    (CallFunction|ActivateEffects IsMain)
    (Utilities|FlowControl|Delay (Utilities|Struct|BreakStruct_WeaponShotParam (Variables|-Shooting|GetMainShotParam)))
    (Variables|Default|SetIsFire true)
    (else
      (Variables|Default|SetIsFire false)
      (CallFunction|ActivateEffects IsMain)
      (Utilities|FlowControl|Delay (Utilities|Struct|BreakStruct_WeaponShotParam (Variables|-Shooting|GetAltShotParam)))
      (Variables|Default|SetIsFire true))))

(event Custom|ActivateEffects
  (params (IsMain :type Boolean))
  (if IsMain
    (Components|Activation|Activate (Variables|Default|GetMain_ShotSound) true)
    (else
      (Components|Activation|Activate (Variables|Default|GetAlt_ShotSound) true))))

(event Custom|PushEnemy
  (params (HitActor :type Actor%20Object%20Reference))
  (Utilities|IsValid HitActor
    (:Is%20Valid
      (Transformation|SetActorRelativeLocation HitActor (+ (Transformation|GetActorLocation HitActor) (* (Transformation|GetActorForwardVector (Game|GetPlayerCameraManager 0)) 1e+02)) true))))

(event EventBeginPlay
  (Variables|-Ammo|SetCurrentAmmo_Main (Variables|-Ammo|GetClipAmmo_Main)))

(event EventTick
  (params (DeltaSeconds :type Float%20%28single-precision%29)))

(fn ConstructionScript)

(fn MakeTraceShot
  (params (IsMain :type Boolean))
  (bind _returnvalue (Game|GetPlayerCameraManager 0))
  (bind _returnvalue_2 (Game|GetPlayerController 0))
  (bind _self self)
  (bind _mainshotparam (Variables|-Shooting|GetMainShotParam))
  (bind _altshotparam (Variables|-Shooting|GetAltShotParam))
  (bind _mainshotparam_2 (Variables|-Shooting|GetMainShotParam))
  (bind _altshotparam_2 (Variables|-Shooting|GetAltShotParam))
  (bind (_range _scatter _projtectileradius) (Utilities|Struct|BreakStruct_WeaponShotParam _mainshotparam_2))
  (bind (_range_2 _scatter_2 _projtectileradius_2) (Utilities|Struct|BreakStruct_WeaponShotParam _altshotparam_2))
  (bind _damage (Utilities|Struct|BreakStruct_WeaponShotParam _altshotparam))
  (bind _damage_2 (Utilities|Struct|BreakStruct_WeaponShotParam _mainshotparam))
  (bind _returnvalue_3 (Camera|GetCameraLocation _returnvalue))
  (bind _returnvalue_4 (select IsMain _damage_2 _damage))
  (bind _outhit (Collision|SphereTraceByChannel _returnvalue_3 (+ _returnvalue_3 (* (Math|Random|RandomUnitVectorinConeinDegrees (Transformation|GetActorForwardVector _returnvalue) (select IsMain _scatter _scatter_2)) (select IsMain _range _range_2))) (select IsMain _projtectileradius _projtectileradius_2) "TraceTypeQuery1" true 0 "None" true "(R=1.000000,G=0.000000,B=0.000000,A=1.000000)" "(R=0.000000,G=1.000000,B=0.000000,A=1.000000)" 2.0))
  (Rendering|Debug|DrawDebugLine (Transformation|GetWorldLocation (select IsMain (Variables|Default|GetMain_Dir) (Variables|Default|GetAlt_Dir))) (select (.bBlockingHit (Collision|BreakHitResult _outhit)) (.ImpactPoint (Collision|BreakHitResult _outhit)) (.TraceEnd (Collision|BreakHitResult _outhit))) "(R=0.255208,G=0.255208,B=0.255208,A=1.000000)" 0.02 1.0)
  (Game|SpawnActorfromClass "/Game/-RLS_Project/Environment/ImpactEffect/BP_ImpactEffect.BP_ImpactEffect_C" (Math|Transform|MakeTransform (select (.bBlockingHit (Collision|BreakHitResult _outhit)) (.ImpactPoint (Collision|BreakHitResult _outhit)) (.TraceEnd (Collision|BreakHitResult _outhit))) "0, 0, 0" "1,1,1") "Undefined" 0 _outhit 0)
  (if (Utilities|Name|Equal(Name) (.HitBoneName (Collision|BreakHitResult _outhit)) "head")
    (Game|Damage|ApplyPointDamage (.HitActor (Collision|BreakHitResult _outhit)) (* _returnvalue_4 2.0) (Math|Vector|Normalize (- (.TraceEnd (Collision|BreakHitResult _outhit)) (.TraceStart (Collision|BreakHitResult _outhit)))) _outhit _returnvalue_2 _self (select IsMain (.Damage_Type (Utilities|Struct|BreakStruct_WeaponShotParam (Variables|-Shooting|GetMainShotParam))) (.Damage_Type (Utilities|Struct|BreakStruct_WeaponShotParam (Variables|-Shooting|GetAltShotParam)))))
    (Game|SpawnActorfromClass "/Game/-RLS_Project/Environment/Worldtext/BP_CriticalHitText.BP_CriticalHitText_C" (Math|Transform|MakeTransform (+ (select (.bBlockingHit (Collision|BreakHitResult _outhit)) (.ImpactPoint (Collision|BreakHitResult _outhit)) (.TraceEnd (Collision|BreakHitResult _outhit))) "0,25.000000,50.000000") (Math|Rotator|FindLookatRotation (select (.bBlockingHit (Collision|BreakHitResult _outhit)) (.ImpactPoint (Collision|BreakHitResult _outhit)) (.TraceEnd (Collision|BreakHitResult _outhit))) (Camera|GetCameraLocation (Game|GetPlayerCameraManager 0))) "1,1,1") "Undefined" 0 0)
    (else
      (Game|Damage|ApplyPointDamage (.HitActor (Collision|BreakHitResult _outhit)) _returnvalue_4 (Math|Vector|Normalize (- (.TraceEnd (Collision|BreakHitResult _outhit)) (.TraceStart (Collision|BreakHitResult _outhit)))) _outhit _returnvalue_2 _self))))

(fn TrySpendAmmo
  (params (IsMain :type Boolean))
  (if (not (Variables|-Ammo|GetIsInfinityAmmo))
    (if (> (select IsMain (Variables|-Ammo|GetCurrentAmmo_Main) (Variables|-Ammo|GetCurrentAmmo_Alt)) 0)
      (Math|Integer|DecrementInt (select IsMain (Variables|-Ammo|GetCurrentAmmo_Main) (Variables|-Ammo|GetCurrentAmmo_Alt))
        (:%20%20
          (CallFunction|SendAmmoInfo)
          (Default|CallOnShot)
          (return true)))
      (else
        (return false)))
    (else
      (Default|CallOnShot)
      (return true))))

(fn TryReload
  (if (and (!= (Variables|-Ammo|GetCurrentAmmo_Main) (Variables|-Ammo|GetClipAmmo_Main)) (!= (Variables|-Ammo|GetTotalAmmo_Main) 0))
    (return true)
    (else
      (return false))))

(fn SendAmmoInfo
  (Default|CallOnAmmoChanged (Variables|-Ammo|GetCurrentAmmo_Main) (Variables|-Ammo|GetTotalAmmo_Main) (Variables|-Ammo|GetCurrentAmmo_Alt) (Variables|-Ammo|GetClipAmmo_Main)))

(fn Reload
  (Variables|-Ammo|SetTotalAmmo_Main (+ (Variables|-Ammo|GetCurrentAmmo_Main) (Variables|-Ammo|GetTotalAmmo_Main)))
  (Variables|-Ammo|SetCurrentAmmo_Main 0)
  (if (>= (Variables|-Ammo|GetTotalAmmo_Main) (Variables|-Ammo|GetClipAmmo_Main))
    (Variables|-Ammo|SetTotalAmmo_Main (- (Variables|-Ammo|GetTotalAmmo_Main) (Variables|-Ammo|GetClipAmmo_Main)))
    (Variables|-Ammo|SetCurrentAmmo_Main (Variables|-Ammo|GetClipAmmo_Main))
    (CallFunction|SendAmmoInfo)
    (else
      (Variables|-Ammo|SetCurrentAmmo_Main (Variables|-Ammo|GetTotalAmmo_Main))
      (Variables|-Ammo|SetTotalAmmo_Main 0))))

(fn AddAmmo
  (params (Amount :type Integer) (IsMain :type Boolean) (WeaponChoose :type E_WeaponChoose%20Enum :default "NewEnumerator0"))
  (Utilities|FlowControl|Sequence
    (:then_0
      (if IsMain
        (Variables|-Ammo|SetTotalAmmo_Main (+ (Variables|-Ammo|GetTotalAmmo_Main) Amount))
        (else
          (Variables|-Ammo|SetCurrentAmmo_Alt (+ (Variables|-Ammo|GetCurrentAmmo_Alt) Amount)))))
    (:then_1
      (if (Utilities|Enum|Equal(Enum) WeaponChoose (Variables|Default|GetWeaponChoose))
        (CallFunction|SendAmmoInfo)))))

(fn TryMakeShot
  (params (IsMain :type Boolean))
  (if (Variables|Default|GetIsFire)
    (return true)))

(fn StopShoot)