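; M16 weapon Blueprint that adds automatic hitscan fire on top of its parent weapon class.
; When the parent's TryMakeShot passes for a main shot, it fires at once and starts a looping timer paced by the main cooldown.
; Each tick spends ammo, makes a trace shot and updates fire-rate control.
; StopShoot or a failed ammo spend clears the timer.
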(event Custom|StartBurst
  (CallFunction|OneShot)
  (bind _returnvalue (Utilities|Time|SetTimerbyEvent (delegate Custom|OneShot) (Utilities|Struct|BreakStruct_WeaponShotParam (Variables|Default|GetMainShotParam)) true))
  (Variables|Default|SetBurstHandle_Main _returnvalue))

(event Custom|OneShot
  (bind _result (CallFunction|TrySpendAmmo true))
  (if _result
    (CallFunction|MakeTraceShot true)
    (CallFunction|FireRateControl true)
    (else
      (CallFunction|StopBurst))))

(event Custom|StopBurst
  (Utilities|Time|ClearandInvalidateTimerbyHandle (Variables|Default|GetBurstHandle_Main)))

(fn ConstructionScript
  (|CallParentFunction))

(fn TryMakeShot
  (params (IsMain :type Boolean))
  (bind _result (|CallParentFunction false))
  (if _result
    (if IsMain
      (CallFunction|StartBurst))))

(fn StopShoot
  (|CallParentFunction)
  (CallFunction|StopBurst))