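; Shotgun weapon Blueprint that fires timed volleys of pellet trace shots when a main-fire attempt succeeds.
; MakeShotGun spends ammo, applies fire rate control, then fires immediately and starts a looping timer that repeats MakeVolley until the volley count is reached.
; Each volley widens the alt-shot scatter from its cached BeginPlay value before tracing every pellet.
; Alt fire is unwired: TryMakeShot only triggers main fire.
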(event Custom|MakeShotGun
  (params (IsMain :type Boolean))
  (bind _result (CallFunction|TrySpendAmmo IsMain))
  (if _result
    (CallFunction|FireRateControl IsMain)
    (Variables|Default|SetCurrentVolleyIndex 0)
    (bind _returnvalue (Utilities|Time|SetTimerbyEvent (EventDispatchers|CreateEvent :!event Custom|MakeVolley) (Variables|Default|GetVolleyTime) true))
    (Variables|Default|SetVolleyHandle _returnvalue)
    (CallFunction|MakeVolley)))

(event Custom|MakeVolley
  (Utilities|FlowControl|Sequence
    (:then_0
      (Utilities|Struct|SetmembersinStruct_WeaponShotParam (Variables|Default|GetAltShotParam) (+ (Variables|Default|GetAltScatterParam) (* (Variables|Default|GetCurrentVolleyIndex) (Variables|Default|GetAltScatterDelta))))
      (for _index (range 1 (Variables|Default|GetPelletAmount))
        (CallFunction|MakeTraceShot (stale Custom|MakeShotGun IsMain))))
    (:then_1
      (bind _result (Math|Integer|IncrementInt (Variables|Default|GetCurrentVolleyIndex))
        (:%20%20
          (if (>= _result (Variables|Default|GetVolleyAmount))
            (Utilities|Time|ClearandInvalidateTimerbyHandle (Variables|Default|GetVolleyHandle))))))))

(event EventBeginPlay
  (|CallParentFunction)
  (Variables|Default|SetAltScatterParam (.Scatter (Utilities|Struct|BreakStruct_WeaponShotParam (Variables|Default|GetAltShotParam)))))

(fn ConstructionScript
  (|CallParentFunction))

(fn TryMakeShot
  (params (IsMain :type Boolean))
  (bind _result (|CallParentFunction false))
  (if _result
    (if IsMain
      (CallFunction|MakeShotGun true))))