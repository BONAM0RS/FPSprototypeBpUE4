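; Sniper weapon Blueprint that fires trace shots in two modes: a main shot and a scope shot.
; It overrides TryMakeShot, runs the parent check, then routes to MakeShot or MakeScopeShot based on IsMain.
; Both events spend ammo first, then call the shared trace and fire-rate functions with a flag identifying the mode.
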(event Custom|MakeShot
  (bind _result (CallFunction|TrySpendAmmo true))
  (if _result
    (CallFunction|MakeTraceShot true)
    (CallFunction|FireRateControl true)))

(event Custom|MakeScopeShot
  (bind _result (CallFunction|TrySpendAmmo true))
  (if _result
    (CallFunction|MakeTraceShot false)
    (CallFunction|FireRateControl false)))

(fn ConstructionScript
  (|CallParentFunction))

(fn TryMakeShot
  (params (IsMain :type Boolean))
  (bind _result (|CallParentFunction false))
  (if _result
    (if IsMain
      (CallFunction|MakeShot)
      (else
        (CallFunction|MakeScopeShot)))))