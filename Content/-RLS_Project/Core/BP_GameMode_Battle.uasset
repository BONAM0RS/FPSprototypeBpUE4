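; Battle game mode that builds a run at BeginPlay by chaining streamed level instances, with the room count set by the game instance's difficulty.
; Each random level, never repeating the previous pick, loads at a BP_LevelAnchor's location, and that anchor is then destroyed.
; Each level's OnLevelShown event triggers the next spawn until the count is reached, then the boss level and finally the end level load.
; Failed loads retry recursively.
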(event Custom|FindNextSpawnPoint
  (bind _outactors (Actor|GetAllActorsOfClass "/Game/-RLS_Project/Environment/BP_LevelAnchor.BP_LevelAnchor_C"))
  (Variables|Default|SetNextSpawnPoint (Transformation|GetActorLocation (Utilities|Array|Get(acopy) _outactors)))
  (Actor|DestroyActor (Utilities|Array|Get(acopy) _outactors)))

(event Custom|SpawnNextLevel
  (if (< (Variables|Default|GetCurrentLevelAmount) (Variables|Default|GetTotalLevelAmount))
    (bind _output_get (Variables|Default|SetRandomCurrentLevel (.OutIndex (Utilities|Array|Random (Variables|Default|GetRandomLevels)))))
    (if (!= _output_get (Variables|Default|GetLastCurrentLevel))
      (bind _output_get_2 (Variables|Default|SetLastCurrentLevel (Variables|Default|GetRandomCurrentLevel)))
      (CallFunction|FindNextSpawnPoint)
      (bind (_boutsuccess _returnvalue) (Class|LevelStreamingDynamic|LoadLevelInstancebySoftObjectPtr (Utilities|Array|Get(acopy) (Variables|Default|GetRandomLevels) _output_get_2) (Variables|Default|GetNextSpawnPoint) "0, 0, 0"))
      (if _boutsuccess
        (EventDispatchers|BindEventtoOnLevelShown _returnvalue (delegate Custom|AddLevel))
        (else
          (CallFunction|SpawnNextLevel)))
      (else
        (CallFunction|SpawnNextLevel)))
    (else
      (CallFunction|FindNextSpawnPoint)
      (bind (_boutsuccess_2 _returnvalue_2) (Class|LevelStreamingDynamic|LoadLevelInstancebySoftObjectPtr (Variables|Default|GetBoss_Level) (Variables|Default|GetNextSpawnPoint) "0, 0, 0"))
      (if _boutsuccess_2
        (EventDispatchers|BindEventtoOnLevelShown _returnvalue_2 (delegate Custom|SpawnEndLevel))
        (else
          (CallFunction|SpawnNextLevel))))))

(event Custom|AddLevel
  (Math|Integer|IncrementInt (Variables|Default|GetCurrentLevelAmount)
    (:%20%20
      (CallFunction|SpawnNextLevel))))

(event Custom|SpawnEndLevel
  (CallFunction|FindNextSpawnPoint)
  (Class|LevelStreamingDynamic|LoadLevelInstancebySoftObjectPtr (Variables|Default|GetEnd_Level) (Variables|Default|GetNextSpawnPoint) "0, 0, 0"))

(event EventBeginPlay
  (Variables|Default|SetTotalLevelAmount (Utilities|Select :Index (Variables|/Game/-RLS_Project/Core/BP_GameInstance.BP_GameInstance_C|GetGameDifficulty (.AsBP%20Game%20Instance (Utilities|Casting|CastToBP_GameInstance (Game|GetGameInstance)))) :Option%200 3 :Option%201 4 :Option%202 5))
  (CallFunction|SpawnNextLevel))

(fn ConstructionScript
  (|CallParentFunction))