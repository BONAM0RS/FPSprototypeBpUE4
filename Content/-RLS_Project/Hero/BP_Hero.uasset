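; First-person player character that handles movement, stamina-limited sprint, weapons, object grabbing and interaction.
; Spawns weapons on the Arms socket, switches them with montages locked by an animation flag, and binds the active weapon's events to recoil and HUD.
; Tick drives the physics handle, a sphere trace for interactables and gated scope updates.
; Camera modifiers convey sprint, scope, low HP and death, with vitality events updating the HUD and triggering the death screen.
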(event OnChangedHP(BP_VitalityComponent)
  (params (CurrentHP :type Float%20%28single-precision%29) (TotalHP :type Float%20%28single-precision%29))
  ;[1 1 1] Vitality Component
  (Default|SetHP (Variables|Default|GetUI) CurrentHP TotalHP)
  (CallFunction|ActivateCamModLowHP (< (/ CurrentHP TotalHP) 0.3)))

(event OnDied(BP_VitalityComponent)
  ;[1 1 1] Vitality Component
  (Utilities|FlowControl|Sequence
    (:then_0
      (CameraModifier|DisableModifier (Variables|Default|GetCamMod_LowHP) true)
      (CallFunction|ActivateDeathCamMod))
    (:then_1
      (for _array_element (Variables|-Weapon|GetWeapons)
        (Actor|DestroyActor _array_element)))
    (:then_2
      (Widget|RemovefromParent (Variables|Default|GetUI))
      (Default|ShowDeathScreen (Variables|Default|GetUI_DeathScreen)))
    (:then_3
      (Actor|DestroyActor))))

(event Custom|Spawn%20Weapons
  ;[1 1 1] Weapon Process
  (for _array_element (Variables|-Weapon|GetWeaponClasses)
    (bind _returnvalue (Game|SpawnActorfromClass _array_element (Math|Transform|MakeTransform "0, 0, 0" "0, 0, 0" "0.000000,0.000000,0.000000") "AlwaysSpawn" 0 0))
    (bind _returnvalue_2 (Utilities|Array|Add (Variables|-Weapon|GetWeapons) _returnvalue))
    (Transformation|AttachComponentToComponent _returnvalue (Variables|Default|GetArms) "gun_rSocket" "SnapToTarget" "SnapToTarget" "SnapToTarget" true)
    (CallFunction|ActivateWeapon _returnvalue false)))

(event Custom|OnWeaponShot
  ;[1 1 1] Weapon Process
  (Animation|Montage|PlayMontage (Variables|Default|GetArms) (.OutItem (Utilities|Array|Random (Variables|/Game/-RLS_Project/Weapons/BP_Weapon_Base.BP_Weapon_Base_C|GetShotMontages (Variables|-Weapon|GetCurrentWeapon))))
    (:then
      (if (not (Variables|Default|GetIsScope))
        (Pawn|Input|AddControllerPitchInput -0.5)
        (Pawn|Input|AddControllerYawInput (Math|Random|RandomFloatinRange -0.5 0.5))))))

(event Custom|CloseScopeTick
  ;[1 1 1] Grab Process
  (Utilities|FlowControl|Gate true) ; enters at Close
)

(event Custom|ShowShotgunHandReload
  ;[1 1 1] Weapon Process
  (Components|SkinnedMesh|UnHideBonebyName (Variables|Default|GetArms) "clavicle_l"))

(event Custom|ActivateDeathCamMod
  ;[1 1 1] Camera Modifier
  (CameraModifier|EnableModifier (Variables|Default|GetCamMod_Death)))

(event Custom|SelectWeaponByIndex
  (params (Index :type Integer))
  ;[1 1 1] Weapon Process
  (Utilities|IsValid (Variables|-Weapon|GetCurrentWeapon)
    (:Is%20Valid
      (if (not (Variables|Default|GetIsAnimBlock))
        (Variables|Default|SetIsAnimBlock true)
        (Animation|Montage|PlayMontage (Variables|Default|GetArms) (Variables|/Game/-RLS_Project/Weapons/BP_Weapon_Base.BP_Weapon_Base_C|GetHolsterMontage (Variables|-Weapon|GetCurrentWeapon))
          (:OnBlendOut
            (Utilities|FlowControl|Sequence :!label _label
              (:then_0
                (Utilities|IsValid (Variables|-Weapon|GetCurrentWeapon)
                  (:Is%20Valid
                    (CallFunction|ActivateWeapon (Variables|-Weapon|GetCurrentWeapon) false))))
              (:then_1
                (if (Utilities|Array|IsValidIndex (Variables|-Weapon|GetWeapons) Index)
                  (bind _output_get (Variables|-Weapon|SetCurrentWeapon (Utilities|Array|Get(acopy) (Variables|-Weapon|GetWeapons) Index)))
                  (Variables|Default|SetCurrentWeaponInt Index)
                  (CallFunction|ActivateWeapon _output_get true)
                  (|PrepareWeapon)
                  (else
                    (CallFunction|SelectWeaponbyIndex))))
              (:then_2
                (Animation|Montage|PlayMontage (Variables|Default|GetArms) (Variables|/Game/-RLS_Project/Weapons/BP_Weapon_Base.BP_Weapon_Base_C|GetEquipMontage (Variables|-Weapon|GetCurrentWeapon))
                  (:OnBlendOut
                    (Variables|Default|SetIsAnimBlock false)))))))))
    (:Is%20Not%20Valid
      (goto _label))))

(event Custom|ChangeStamina
  (bind _staminapertick (Variables|-Stamina|GetStaminaPerTick))
  ;[1 1 1] Sprint Process
  (bind _output_get (Variables|-Stamina|SetCurrentStamina (Math|Float|Clamp(Float) (+ (Variables|-Stamina|GetCurrentStamina) (select (Variables|-Stamina|GetIsSprint) (* _staminapertick (Variables|-Stamina|GetStaminaCost)) (* (Variables|-Stamina|GetStaminaRegen) _staminapertick))) 0.0 (Variables|-Stamina|GetTotalStamina))))
  (Default|SetStamina (Variables|Default|GetUI) _output_get (Variables|-Stamina|GetTotalStamina))
  (if (or (== (Variables|-Stamina|GetCurrentStamina) 0.0) (<= (Input|AxisValues|GetMoveForward) 0.0))
    (CallFunction|StopSprint)))

(event Custom|StopSprint
  ;[1 1 1] Sprint Process
  (if (Variables|-Stamina|GetIsSprint)
    (Variables|-Stamina|SetIsSprint false)
    (Variables|/Script/Engine.CharacterMovementComponent|SetMaxWalkSpeed (Variables|Character|GetCharacterMovement) (Variables|Default|GetDefaultWalkSpeed))
    (CameraModifier|DisableModifier (Variables|-Stamina|GetCamMod_Sprint) false)
    (CameraShakes|StopCameraShake (Game|GetPlayerCameraManager 0) (Variables|-Stamina|GetCamShake_Sprint) false)))

(event Custom|ActivateCamModLowHP
  (params (CheckHP :type Boolean))
  (bind _cammod_lowhp (Variables|Default|GetCamMod_LowHP))
  ;[1 1 1] Camera Modifier
  (if CheckHP
    (CameraModifier|EnableModifier _cammod_lowhp)
    (else
      (CameraModifier|DisableModifier _cammod_lowhp false))))

(event Custom|ActivateWeapon
  (params (Weapon :type BP%20Weapon%20Base%20Object%20Reference) (OnOff :type Boolean))
  ;[1 1 1] Weapon Process
  (Collision|SetActorEnableCollision Weapon OnOff)
  (Rendering|SetActorHiddenInGame Weapon (not OnOff))
  (if (== (Variables|Default|GetCurrentWeaponInt) 0)
    (Components|SkinnedMesh|HideBonebyName (Variables|Default|GetArms) "clavicle_l" "PBO_None")
    (else
      (Components|SkinnedMesh|UnHideBonebyName (Variables|Default|GetArms) "clavicle_l"))))

(event Custom|InteractTrace
  (bind _camera (Variables|Default|GetCamera))
  (bind _returnvalue (Transformation|GetWorldLocation _camera))
  ;[1 1 1] Interact
  (bind _outhit (Collision|SphereTraceByChannel _returnvalue (+ _returnvalue (* (Math|Vector|GetForwardVector _camera) 5e+02)) 2.0 "TraceTypeQuery1" true 0 "None" true "(R=1.000000,G=0.697965,B=0.000000,A=1.000000)" "(R=0.000000,G=1.000000,B=0.000000,A=1.000000)" 0.1))
  (Utilities|IsValid (.HitActor (Collision|BreakHitResult _outhit))
    (:Is%20Valid
      (if (Utilities|DoesObjectImplementInterface (.HitActor (Collision|BreakHitResult _outhit)) "/Game/-RLS_Project/Environment/Interactable/BPI_Interactable.BPI_Interactable_C")
        (if (not (Variables|Default|GetisFocus))
          (Class|BPIInteractable|OnFocus(Message) (.HitActor (Collision|BreakHitResult _outhit)) true)
          (bind _output_get (Variables|Default|SetCurrentInteractedActor (.HitActor (Collision|BreakHitResult _outhit))))
          (Variables|Default|SetisFocus true)
          (bind _infostring (Class|BPIInteractable|GetInfo(Message) _output_get))
          (Development|PrintString _infostring))
        (else
          (if (Variables|Default|GetisFocus) :!label _label
            (Utilities|IsValid (Variables|Default|GetCurrentInteractedActor)
              (:Is%20Valid
                (Class|BPIInteractable|OnFocus(Message) (Variables|Default|GetCurrentInteractedActor) false))
              (:Is%20Not%20Valid
                _))
            (Variables|Default|SetCurrentInteractedActor 0)
            (Variables|Default|SetisFocus false)))))
    (:Is%20Not%20Valid
      (goto _label))))

(event Custom|HideShotgunHandReload
  ;[1 1 1] Weapon Process
  (Components|SkinnedMesh|HideBonebyName (Variables|Default|GetArms) "clavicle_l" "PBO_None"))

(event Custom|OpenScopeTick
  ;[1 1 1] Grab Process
  (Utilities|FlowControl|Gate true) ; enters at Open
)

(event EventBeginPlay
  (bind _bp_vitalitycomponent (Variables|Default|GetBP_VitalityComponent))
  (bind _totalhp (Variables|/Game/-RLS_Project/Components/BP_VitalityComponent.BP_VitalityComponent_C|GetTotalHP _bp_vitalitycomponent))
  (Utilities|Casting|CastToPlayerController (Pawn|GetController))
  (Variables|Default|SetDefaultWalkSpeed (Variables|/Script/Engine.CharacterMovementComponent|GetMaxWalkSpeed (Variables|Character|GetCharacterMovement)))
  (bind _returnvalue (UserInterface|CreateWidget "/Game/-RLS_Project/UI/Widgets/WBP_UI.WBP_UI_C"))
  (bind _output_get (Variables|Default|SetUI _returnvalue))
  (UserInterface|Viewport|AddtoViewport _output_get 0)
  (CallFunction|SpawnWeapons)
  (CallFunction|SelectWeaponbyIndex)
  (CallFunction|CreateCamMods)
  (bind _returnvalue_2 (Utilities|Time|SetTimerbyEvent (EventDispatchers|CreateEvent :!event Custom|ChangeStamina) (Variables|-Stamina|GetStaminaPerTick) true))
  (Variables|-Stamina|SetStaminaTimerHandle _returnvalue_2)
  (Variables|-Stamina|SetCurrentStamina (Variables|-Stamina|GetTotalStamina))
  (bind _output_get_2 (Variables|Default|SetCurrentHP _totalhp))
  (Default|SetHP (Variables|Default|GetUI) _output_get_2 _totalhp)
  (Components|SkinnedMesh|HideBonebyName (Variables|Character|GetMesh) "clavicle_l" "PBO_None")
  (Components|SkinnedMesh|HideBonebyName (Variables|Character|GetMesh) "clavicle_r" "PBO_None")
  (bind _returnvalue_3 (UserInterface|CreateWidget "/Game/-RLS_Project/UI/Widgets/WBP_DeathScreen.WBP_DeathScreen_C"))
  (Variables|Default|SetUI_DeathScreen _returnvalue_3)
  (bind _returnvalue_4 (UserInterface|CreateWidget "/Game/-RLS_Project/UI/Widgets/WBP_WinScreen.WBP_WinScreen_C"))
  (Variables|Default|SetUI_WinScreen _returnvalue_4))

(event EventTick
  (params (DeltaSeconds :type Float%20%28single-precision%29))
  (bind _grabpoint (Variables|Default|GetGrabPoint))
  ;[1 1 1] Grab Process
  (Class|PhysicsHandleComponent|SetTargetLocationandRotation (Variables|Default|GetPhysicsHandle) (Transformation|GetWorldLocation _grabpoint) (Transformation|GetWorldRotation _grabpoint))
  (CallFunction|InteractTrace)
  (Utilities|FlowControl|Gate true
    (:Exit
      (bind _asbp_scope_cam_mod (Utilities|Casting|CastToBP_Scope_CamMod (Variables|Default|GetCamMod_Scope)))
      (Variables|/Game/-RLS_Project/Hero/CameraModifiers/BP_Scope_CamMod.BP_Scope_CamMod_C|SetWeaponTransform _asbp_scope_cam_mod (Transformation|GetSocketTransform (Variables|/Game/-RLS_Project/Weapons/BP_Weapon_Base.BP_Weapon_Base_C|GetWeaponMesh (Variables|-Weapon|GetCurrentWeapon)) "ScopeSocket" "RTS_World")))))

(event Input|ActionEvents|InputActionCrouch
  (params (Key :type Key%20Structure :default "None"))
  ;[1 1 1] Basic Inputs
  (:Pressed
    (Character|Crouch))
  (:Released
    (Character|UnCrouch)))

(event Input|ActionEvents|InputActionJump
  (params (Key :type Key%20Structure :default "None"))
  ;[1 1 1] Basic Inputs
  (:Pressed
    (Character|Jump))
  (:Released
    (Character|StopJumping)))

(event Input|ActionEvents|InputActionInteract
  (params (Key :type Key%20Structure :default "None"))
  (bind _currentinteractedactor (Variables|Default|GetCurrentInteractedActor))
  ;[1 1 1] Interact
  (:Pressed
    (Utilities|IsValid _currentinteractedactor
      (:Is%20Valid
        (Class|BPIInteractable|Interact(Message) _currentinteractedactor)))))

(event Input|ActionEvents|InputActionSelectWeapon_02
  (params (Key :type Key%20Structure :default "None"))
  ;[1 1 1] Weapon Process
  (:Pressed
    (if (!= (Variables|Default|GetCurrentWeaponInt) 1)
      (CallFunction|SelectWeaponbyIndex 1))))

(event Input|ActionEvents|InputActionSelectWeapon_03
  (params (Key :type Key%20Structure :default "None"))
  ;[1 1 1] Weapon Process
  (:Pressed
    (if (!= (Variables|Default|GetCurrentWeaponInt) 2)
      (CallFunction|SelectWeaponbyIndex 2))))

(event Input|ActionEvents|InputActionSelectWeapon_05
  (params (Key :type Key%20Structure :default "None"))
  ;[1 1 1] Weapon Process
  (:Pressed
    (if (!= (Variables|Default|GetCurrentWeaponInt) 4)
      (CallFunction|SelectWeaponbyIndex 4))))

(event Input|ActionEvents|InputActionSelectWeapon_06
  (params (Key :type Key%20Structure :default "None"))
  ;[1 1 1] Weapon Process
  (:Pressed
    (if (!= (Variables|Default|GetCurrentWeaponInt) 5)
      (CallFunction|SelectWeaponbyIndex 5))))

(event Input|ActionEvents|InputActionSprint
  (params (Key :type Key%20Structure :default "None"))
  (bind _returnvalue (Game|GetPlayerCameraManager 0))
  (bind _charactermovement (Variables|Character|GetCharacterMovement))
  (bind _cammod_sprint (Variables|-Stamina|GetCamMod_Sprint))
  ;[1 1 1] Sprint Process
  (:Pressed
    (if (Math|Boolean|ANDBoolean (not (Variables|-Stamina|GetIsSprint)) (> (Variables|-Stamina|GetCurrentStamina) 0.0) (>= (Input|AxisValues|GetMoveForward) 0.5))
      (if (not (Variables|Default|GetIsScope))
        (Variables|-Stamina|SetIsSprint true)
        (Variables|/Script/Engine.CharacterMovementComponent|SetMaxWalkSpeed _charactermovement 9e+02)
        (CameraModifier|EnableModifier _cammod_sprint)
        (bind _returnvalue_2 (CameraShakes|StartCameraShake _returnvalue "/Game/-RLS_Project/Hero/CameraModifiers/BP_Sprint_CamShake_Matinee.BP_Sprint_CamShake_Matinee_C" 1.0 "CameraLocal" "0, 0, 0"))
        (Variables|-Stamina|SetCamShake_Sprint _returnvalue_2))))
  (:Released
    (if (Variables|-Stamina|GetIsSprint)
      (Variables|-Stamina|SetIsSprint false)
      (Variables|/Script/Engine.CharacterMovementComponent|SetMaxWalkSpeed _charactermovement (Variables|Default|GetDefaultWalkSpeed))
      (CameraModifier|DisableModifier _cammod_sprint false)
      (CameraShakes|StopCameraShake _returnvalue (Variables|-Stamina|GetCamShake_Sprint) false))))

(event Input|ActionEvents|InputActionSelectWeapon_01
  (params (Key :type Key%20Structure :default "None"))
  ;[1 1 1] Weapon Process
  (:Pressed
    (if (!= (Variables|Default|GetCurrentWeaponInt) 0)
      (CallFunction|SelectWeaponbyIndex))))

(event Input|ActionEvents|InputActionSelectWeapon_04
  (params (Key :type Key%20Structure :default "None"))
  ;[1 1 1] Weapon Process
  (:Pressed
    (if (!= (Variables|Default|GetCurrentWeaponInt) 3)
      (CallFunction|SelectWeaponbyIndex 3))))

(event Input|ActionEvents|InputActionMainAttack
  (params (Key :type Key%20Structure :default "None"))
  (bind _currentweapon (Variables|-Weapon|GetCurrentWeapon))
  ;[1 1 1] Weapon Process
  (:Pressed
    (if (not (Variables|Default|GetIsAnimBlock))
      (if (not (Variables|Default|GetIsScope))
        (Default|TryMakeShot _currentweapon true)
        (else
          (Default|TryMakeShot _currentweapon false)))))
  (:Released
    (Default|StopShoot (Variables|-Weapon|GetCurrentWeapon))))

(event Input|ActionEvents|InputActionAltAttack
  (params (Key :type Key%20Structure :default "None"))
  (bind _ui (Variables|Default|GetUI))
  (bind _ui_2 (Variables|Default|GetUI))
  (bind _cammod_scope (Variables|Default|GetCamMod_Scope))
  ;[1 1 1] Weapon Process
  (:Pressed
    (if (not (Variables|Default|GetIsAnimBlock))
      (if (not (Variables|-Stamina|GetIsSprint))
        (if (Variables|/Game/-RLS_Project/Weapons/BP_Weapon_Base.BP_Weapon_Base_C|GetHaveScope (Variables|-Weapon|GetCurrentWeapon))
          (CameraModifier|EnableModifier _cammod_scope)
          (Variables|Default|SetDefaultWalkSpeed (/ (Variables|Default|GetDefaultWalkSpeed) 2.0))
          (Variables|Default|SetIsScope true)
          (CallFunction|OpenScopeTick)
          (if (== (Variables|Default|GetCurrentWeaponInt) 4)
            (Widget|SetVisibility (Variables|/Game/-RLS_Project/UI/Widgets/WBP_UI.WBP_UI_C|GetCanvasPanel—BasicCrosshair _ui_2) "Hidden")
            (Widget|SetVisibility (Variables|/Game/-RLS_Project/UI/Widgets/WBP_UI.WBP_UI_C|GetCanvasPanel—SniperCrosshair _ui_2) "Visible"))
          (else
            (Default|TryMakeShot (Variables|-Weapon|GetCurrentWeapon) false))))))
  (:Released
    (if (Variables|Default|GetIsScope)
      (CameraModifier|DisableModifier _cammod_scope false)
      (Variables|Default|SetDefaultWalkSpeed (* (Variables|Default|GetDefaultWalkSpeed) 2.0))
      (Variables|Default|SetIsScope false)
      (CallFunction|CloseScopeTick)
      (if (== (Variables|Default|GetCurrentWeaponInt) 4)
        (Widget|SetVisibility (Variables|/Game/-RLS_Project/UI/Widgets/WBP_UI.WBP_UI_C|GetCanvasPanel—BasicCrosshair _ui) "Visible")
        (Widget|SetVisibility (Variables|/Game/-RLS_Project/UI/Widgets/WBP_UI.WBP_UI_C|GetCanvasPanel—SniperCrosshair _ui) "Hidden")))))

(event Input|ActionEvents|InputActionReload
  (params (Key :type Key%20Structure :default "None"))
  (bind _currentweapon (Variables|-Weapon|GetCurrentWeapon))
  ;[1 1 1] Weapon Process
  (:Pressed
    (if (!= (Variables|Default|GetCurrentWeaponInt) 5)
      (bind _result (Default|TryReload (Variables|-Weapon|GetCurrentWeapon)))
      (if _result
        (if (not (Variables|Default|GetIsAnimBlock))
          (Variables|Default|SetIsAnimBlock true)
          (Default|WeaponStartReload _currentweapon)
          (Animation|Montage|PlayMontage (Variables|Default|GetArms) (Variables|/Game/-RLS_Project/Weapons/BP_Weapon_Base.BP_Weapon_Base_C|GetReloadMontage _currentweapon)
            (:OnBlendOut
              (Variables|Default|SetIsAnimBlock false))))))))

(event Input|ActionEvents|InputActionGrab
  (params (Key :type Key%20Structure :default "None"))
  (bind _camera (Variables|Default|GetCamera))
  (bind _physicshandle (Variables|Default|GetPhysicsHandle))
  (bind _currentinteractedactor (Variables|Default|GetCurrentInteractedActor))
  (bind _returnvalue (Transformation|GetWorldLocation _camera))
  (bind _returnvalue_2 (Class|PhysicsHandleComponent|GetGrabbedComponent _physicshandle))
  ;[1 1 1] Grab Process
  (:Pressed
    (bind (_outhit _returnvalue_3) (Collision|LineTraceByChannel _returnvalue (+ _returnvalue (* (Math|Vector|GetForwardVector _camera) 1e+03)) "TraceTypeQuery1" false 0 "None"))
    (if _returnvalue_3
      (if (Physics|IsSimulatingPhysics (.HitComponent (Collision|BreakHitResult _outhit)) "None")
        (Physics|Components|PhysicsHandle|GrabComponentatLocationwithRotation (Variables|Default|GetPhysicsHandle) (.HitComponent (Collision|BreakHitResult _outhit)) "None" (Transformation|GetWorldLocation (.HitComponent (Collision|BreakHitResult _outhit))) (Transformation|GetWorldRotation (.HitComponent (Collision|BreakHitResult _outhit))))
        (Utilities|IsValid _currentinteractedactor
          (:Is%20Valid
            (Class|BPIInteractable|Grab(Message) _currentinteractedactor))))))
  (:Released
    (Utilities|IsValid _returnvalue_2
      (:Is%20Valid
        (Physics|AddImpulse _returnvalue_2 (* (Math|Vector|GetForwardVector (Variables|Default|GetCamera)) 1e+03) "None" false)
        (Physics|Components|PhysicsHandle|ReleaseComponent (Variables|Default|GetPhysicsHandle))))))

(event Input|ActionEvents|InputActionThrow
  (params (Key :type Key%20Structure :default "None"))
  (bind _physicshandle (Variables|Default|GetPhysicsHandle))
  (bind _returnvalue (Class|PhysicsHandleComponent|GetGrabbedComponent _physicshandle))
  ;[1 1 1] Grab Process
  (:Pressed
    (Utilities|IsValid _returnvalue
      (:Is%20Valid
        (Physics|AddImpulse _returnvalue (* (Math|Vector|GetForwardVector (Variables|Default|GetCamera)) 2e+05) "None" false)
        (Physics|Components|PhysicsHandle|ReleaseComponent (Variables|Default|GetPhysicsHandle))))))

(event Input|AxisEvents|InputAxisMoveForward
  (params (AxisValue :type Float%20%28single-precision%29))
  ;[1 1 1] Basic Inputs
  (Pawn|Input|AddMovementInput (Math|Vector|GetForwardVector (Math|Rotator|MakeRotator 0.0 0.0 (.yaw (Transformation|GetWorldRotation (Variables|Default|GetCamera))))) AxisValue false))

(event Input|AxisEvents|InputAxisMoveRight
  (params (AxisValue :type Float%20%28single-precision%29))
  ;[1 1 1] Basic Inputs
  (Pawn|Input|AddMovementInput (Math|Vector|GetRightVector (Variables|Default|GetCamera)) AxisValue false))

(event Input|AxisEvents|InputAxisTurn
  (params (AxisValue :type Float%20%28single-precision%29))
  ;[1 1 1] Basic Inputs
  (Variables|Default|SetAxis%20Turn AxisValue)
  (if (Variables|Default|GetIsScope)
    (Pawn|Input|AddControllerYawInput (/ (Variables|Default|GetAxis%20Turn) 2.0))
    (else
      (Pawn|Input|AddControllerYawInput (Variables|Default|GetAxis%20Turn)))))

(event Input|AxisEvents|InputAxisLookUp
  (params (AxisValue :type Float%20%28single-precision%29))
  ;[1 1 1] Basic Inputs
  (Variables|Default|SetAxis%20LookUp AxisValue)
  (if (Variables|Default|GetIsScope)
    (Pawn|Input|AddControllerPitchInput (/ (Variables|Default|GetAxis%20LookUp) 2.0))
    (else
      (Pawn|Input|AddControllerPitchInput (Variables|Default|GetAxis%20LookUp)))))

(fn ConstructionScript)

(fn CreateCamMods
  (Utilities|FlowControl|Sequence
    (:then_0
      (bind _returnvalue (Game|Player|AddNewCameraModifier (Game|GetPlayerCameraManager 0) "/Game/-RLS_Project/Hero/CameraModifiers/BP_Sprint_CamMod.BP_Sprint_CamMod_C"))
      (bind _output_get (Variables|-Stamina|SetCamMod_Sprint _returnvalue))
      (CameraModifier|DisableModifier _output_get true))
    (:then_1
      (bind _returnvalue_2 (Game|Player|AddNewCameraModifier (Game|GetPlayerCameraManager 0) "/Game/-RLS_Project/Hero/CameraModifiers/BP_LowHP_CamMod.BP_LowHP_CamMod_C"))
      (bind _output_get_2 (Variables|Default|SetCamMod_LowHP _returnvalue_2))
      (CameraModifier|DisableModifier _output_get_2 true))
    (:then_2
      (bind _returnvalue_3 (Game|Player|AddNewCameraModifier (Game|GetPlayerCameraManager 0) "/Game/-RLS_Project/Hero/CameraModifiers/BP_Scope_CamMod.BP_Scope_CamMod_C"))
      (bind _output_get_3 (Variables|Default|SetCamMod_Scope _returnvalue_3))
      (CameraModifier|DisableModifier _output_get_3 true))
    (:then_3
      (bind _returnvalue_4 (Game|Player|AddNewCameraModifier (Game|GetPlayerCameraManager 0) "/Game/-RLS_Project/Hero/CameraModifiers/BP_Death_CamMod.BP_Death_CamMod_C"))
      (bind _output_get_4 (Variables|Default|SetCamMod_Death _returnvalue_4))
      (CameraModifier|DisableModifier _output_get_4 true))))

(event Custom|OnAmmoChanged
  (params (CurrentAmmo_Main :type Integer) (TotalAmmo_Main :type Integer) (CurrentAmmo_Alt :type Integer) (ClipAmmo_Main :type Integer))
  (Default|SetAmmo (Variables|Default|GetUI) CurrentAmmo_Main TotalAmmo_Main CurrentAmmo_Alt ClipAmmo_Main (Variables|Default|GetCurrentWeaponInt)))