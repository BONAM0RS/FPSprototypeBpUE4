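; Hero player controller that handles pausing and the pause menu.
; BeginPlay creates the pause menu widget, binds its resume event and sets game-only input.
; The Pause action toggles game pause, menu visibility, mouse cursor and input mode, sharing the resume logic with the menu.
; A settings handler hides the menu's Settings button and shows a settings panel, but this graph neither binds it nor creates that panel.
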(event Custom|OnPauseMenuResume
  (Game|SetGamePaused false)
  (Widget|RemovefromParent (Variables|Default|GetPauseMenu))
  (Variables|Default|SetbShowMouseCursor false)
  (Input|SetInputModeGameOnly self))

(event Custom|OnPauseMenuSettings
  (Widget|SetVisibility (Variables|/Game/-RLS_Project/UI/Widgets/WBP_PauseMenu.WBP_PauseMenu_C|GetButton_Settings (Variables|Default|GetPauseMenu)) "Collapsed")
  (UserInterface|Viewport|AddtoViewport (Variables|Default|GetSettingsPanel) 200))

(event EventBeginPlay
  (bind _returnvalue (UserInterface|CreateWidget "/Game/-RLS_Project/UI/Widgets/WBP_PauseMenu.WBP_PauseMenu_C"))
  (bind _output_get (Variables|Default|SetPauseMenu _returnvalue))
  (EventDispatchers|BindEventtoOnResume _output_get (delegate Custom|OnPauseMenuResume))
  (Input|SetInputModeGameOnly self))

(event Input|ActionEvents|InputActionPause
  (params (Key :type Key%20Structure))
  (bind _self self)
  (:Pressed
    (if (Game|IsGamePaused)
      (Game|SetGamePaused false)
      (Widget|RemovefromParent (Variables|Default|GetPauseMenu))
      (Variables|Default|SetbShowMouseCursor false)
      (Input|SetInputModeGameOnly _self)
      (else
        (Game|SetGamePaused true)
        (UserInterface|Viewport|AddtoViewport (Variables|Default|GetPauseMenu) 100)
        (Variables|Default|SetbShowMouseCursor true)
        (Input|SetInputModeGameandUI _self 0 "DoNotLock" true)))))

(fn ConstructionScript)